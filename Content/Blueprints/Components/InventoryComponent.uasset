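; Inventory component that stores the owner's items as structs, separating key items from usable ones.
; Adding looks up the item's row in DT_GameItems by index, tops up non-full matching stacks, then appends any remainder as a new entry.
; Opening spawns a BP_Inventory actor far below the world with the usable items; closing shuts it.
; Open, close and removal fire events, and helpers check keys, emptiness or replace the list.
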(event `self.ReceiveBeginPlay`
  (bind _asbp_game_instance (cast `/Game/Blueprints/BP_GameInstance` (`GameplayStatics.GetGameInstance`)))
  (set `self.GameInstance` _asbp_game_instance)
  (bind _outrownames (`DataTableFunctionLibrary.GetDataTableRowNames` "/Game/Data/DT_GameItems.DT_GameItems"))
  (set `self.ItemNames` _outrownames))

(fn `AddToInventory`
  (params (Item :type "/Game/Data/ENUM_Items Enum" :default "NewEnumerator0") (Quantity :type Integer))
  (locals (Added :type Boolean) (ToAdd :type Integer) (ItemToAdd :type "/Game/Data/STRUCT_InventoryItem Structure"))
  (bind (_itemindex _name _description _quantity _max _iskey _itemclass) (break `/Game/Data/STRUCT_InventoryItem` (`local.ItemToAdd`)))
  (set `local.ItemToAdd` (`self.RetrieveData` Item Quantity))
  (set `local.ToAdd` Quantity)
  (for (_array_element _array_index) (`self.Items`)
    (bind (_itemindex_2 _name_2 _description_2 _quantity_2 _max_2) (break `/Game/Data/STRUCT_InventoryItem` _array_element))
    (if (and (not (`self.IsItemFull` _array_element)) (== _itemindex_2 (`.ItemIndex_18_04A9D5AC4AACCB80CE078FADF073EE6A` (break `/Game/Data/STRUCT_InventoryItem` (`local.ItemToAdd`)))))
      (bind _output_get (set `local.ToAdd` (- (`local.ToAdd`) (- _max_2 _quantity_2))))
      (bind _returnvalue (<= _output_get 0))
      (if _returnvalue
        (set `local.Added` true))
      (bind (_itemindex_3 _name_3 _description_3 _quantity_3 _max_3 _iskey_2 _itemclass_2) (break `/Game/Data/STRUCT_InventoryItem` _array_element))
      (`KismetArrayLibrary.Array_Set` (`self.Items`) _array_index (make `/Game/Data/STRUCT_InventoryItem` _itemindex_3 _name_3 _description_3 (`KismetMathLibrary.SelectInt` (+ (`local.ToAdd`) _max_3) _max_3 _returnvalue) _max_3 _iskey_2 _itemclass_2))))
  (if (not (`local.Added`))
    (bind _returnvalue_2 (`KismetArrayLibrary.Array_Add` (`self.Items`) (make `/Game/Data/STRUCT_InventoryItem` _itemindex _name _description (`local.ToAdd`) _max _iskey _itemclass)))
    (`KismetSystemLibrary.PrintString` (`KismetStringLibrary.Conv_IntToString` _returnvalue_2))))

(fn `CloseInventory`
  (`/Game/Blueprints/BP_Inventory.Close` (`self.InventoryActor`))
  (`self.OnInventoryClose`)
  (`KismetSystemLibrary.PrintString` "Hello"))

(fn `GetKeyItems`
  (returns (KeyItems :type "Array of /Game/Data/STRUCT_InventoryItem Structure"))
  (locals (TempKeys :type "Array of /Game/Data/STRUCT_InventoryItem Structure"))
  (for _array_element (`self.Items`)
    (if (`self.IsKey` _array_element)
      (`KismetArrayLibrary.Array_Add` (`local.TempKeys`) _array_element)))
  (return (`local.TempKeys`)))

(fn `GetUsableItems`
  (returns (UsableItems :type "Array of /Game/Data/STRUCT_InventoryItem Structure"))
  (locals (TempItems :type "Array of /Game/Data/STRUCT_InventoryItem Structure"))
  (for _array_element (`self.Items`)
    (if (not (`self.IsKey` _array_element))
      (`KismetArrayLibrary.Array_Add` (`local.TempItems`) _array_element)))
  (return (`local.TempItems`)))

(fn `HasKey`
  (params (KeyIndex :type Integer))
  (returns (HasKey :type Boolean))
  (locals (TempHasKey :type Boolean))
  (for _array_element (`self.GetKeyItems`)
    (if (== (`self.GetItemIndex` _array_element) (`local.KeyIndex`))
      (set `local.TempHasKey` true)
      (break)))
  (return (`local.TempHasKey`)))

(fn `IsInventoryEmpty`
  (returns (IsEmpty :type Boolean))
  (return (or (== (`KismetArrayLibrary.Array_Length` (`self.GetUsableItems`)) 0) (== (`KismetArrayLibrary.Array_Length` (`self.Items`)) 0))))

(fn `OpenInventory`
  (bind _returnvalue (`|SpawnActorFromClass` "/Game/Blueprints/BP_Inventory.BP_Inventory_C" (`KismetMathLibrary.MakeTransform` (0.0 0.0 -1000000.0)) "Undefined" "OverrideRootScale" null (`self.GetUsableItems`) self (`self.GameInstance`) null))
  (set `self.InventoryActor` _returnvalue)
  (`self.OnInventoryOpen`))

(fn `RemoveFromInventory`
  (params (Index :type Integer) (Quantity :type Integer))
  (bind (_itemindex _name _description _quantity _max _iskey _itemclass) (break `/Game/Data/STRUCT_InventoryItem` (`|GetArrayItem` (`self.Items`) Index)))
  (bind _returnvalue (- _quantity (`local.Quantity`)))
  (if (== _returnvalue 0)
    (`KismetArrayLibrary.Array_Remove` (`self.Items`) (`local.Index`))
    (else
      (`KismetArrayLibrary.Array_Set` (`self.Items`) (`local.Index`) (make `/Game/Data/STRUCT_InventoryItem` _itemindex _name _description _returnvalue _max _iskey _itemclass))))
  (`self.OnInventoryUpdated`))

(fn `RetrieveData`
  (params (Item :type "/Game/Data/ENUM_Items Enum" :default "NewEnumerator0") (Quantity :type Integer))
  (returns (ItemData :type "/Game/Data/STRUCT_InventoryItem Structure"))
  (bind _returnvalue (`|GetDataTableRow` "/Game/Data/DT_GameItems.DT_GameItems" (`|GetArrayItem` (`self.ItemNames`) (`KismetMathLibrary.Conv_ByteToInt` Item)))
    (:`then`
      (`|VariableSetRef` (`.Quantity_20_29F77E864F14E7BEB05B07BC98EBCE1E` (break `/Game/Data/STRUCT_InventoryItem` _returnvalue)) (`local.Quantity`))
      (return _returnvalue))
    (:`RowNotFound`
      (return))))

(fn `SetInventory`
  (params (NewInventory :type "Array of /Game/Data/STRUCT_InventoryItem Structure"))
  (locals (TempInventory :type "Array of /Game/Data/STRUCT_InventoryItem Structure"))
  (for _array_element NewInventory
    (if (!= (`.ItemIndex_18_04A9D5AC4AACCB80CE078FADF073EE6A` (break `/Game/Data/STRUCT_InventoryItem` _array_element)) 0)
      (`KismetArrayLibrary.Array_Add` (`local.TempInventory`) _array_element)))
  (set `self.Items` (`local.TempInventory`)))