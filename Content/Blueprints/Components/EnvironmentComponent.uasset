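; Environment component that runs the day/night cycle, random weather changes and intermittent ambient sounds.
; A looping timer, scaled by CycleSpeed, advances a clock seeded from local time and feeds BP_LevelLight a mirrored 12-hour daylight alpha.
; Self-recursive delayed events re-roll between two weather states and replay random "environment"-tagged AmbientSounds.
; Sound gathering and light setup are separate entry points not called from BeginPlay.
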(event `self.ReceiveBeginPlay`
  (`self.LoopEnvironmentSounds`)
  (`self.SetLocalTime`)
  (`self.DynamicWeather`)
  (set `self.CurrentWeather` (`self.GetRandomWeather`)))

(event `PlayEnvironmentSounds`
  ;[1 0.7581 0.1451 1 20] Environment Sounds
  (bind _outactors (`GameplayStatics.GetAllActorsOfClassWithTag` "/Script/Engine.AmbientSound" "environment"))
  (set `self.EnvironmentSounds` _outactors))

(event `LoopEnvironmentSounds`
  (bind _outitem (`KismetArrayLibrary.Array_Random` (`self.EnvironmentSounds`)))
  ;[1 0.7581 0.1451 1 20] Environment Sounds
  (`/Engine/EditorBlueprintResources/StandardMacros.IsValid` _outitem
    (:`Is Valid`
      (`AudioComponent.Play` (`AmbientSound.AudioComponent` _outitem) 0.0))
    (:`Is Not Valid`
      _))
  (`KismetSystemLibrary.Delay` (`KismetMathLibrary.RandomFloatInRange` 5.0 20.0))
  (`self.LoopEnvironmentSounds`))

(event `DayCycle`
  ;[1 0.7581 0.1451 1 20] Day Cycle
  (bind _returnvalue (`KismetSystemLibrary.K2_SetTimer` null "UpdateTime" (`self.GetCycleUpdateTime`) true))
  (set `self.Timer_DayCycle` _returnvalue))

(event `DynamicWeather`
  (bind _newweather (`self.GetRandomWeather`))
  (`KismetSystemLibrary.Delay` (`KismetMathLibrary.RandomFloatInRange` 480.0 720.0))
  (if (`|EnumInequality` _newweather (`self.GetCurrentWeather`))
    (set `self.CurrentWeather` _newweather)
    (bind _levellighting (`self.LevelLighting`)
      (:`then`
        (`/Game/Blueprints/Misc/BP_LevelLight.UpdateWeather` _levellighting (`self.GetCurrentWeather`)))
      (:`else`
        _)))
  (`self.DynamicWeather`))

(fn `GetCurrentWeather`
  (returns (Weather :type "/Game/Data/ENUM_Weather Enum"))
  (return (`self.CurrentWeather`)))

(fn `GetCycleUpdateTime`
  (returns (Time :type "Float (double-precision)"))
  (return (/ 1.0 (`self.CycleSpeed`))))

(fn `GetDayLightAlpha`
  (returns (Alpha :type "Float (double-precision)"))
  (bind _returnvalue (/ (`KismetMathLibrary.Conv_IntToDouble` (`self.GetTotalSeconds`)) 43200.0))
  (bind _returnvalue_2 (`KismetMathLibrary.Fraction` _returnvalue))
  (return (`KismetMathLibrary.SelectFloat` _returnvalue_2 (- 1.0 _returnvalue_2) (== (`KismetMathLibrary.FTrunc` _returnvalue) 0))))

(fn `GetRandomWeather`
  (returns (NewWeather :type "/Game/Data/ENUM_Weather Enum"))
  (return (`KismetArrayLibrary.Array_Random` (`|MakeArray` "NewEnumerator0" "NewEnumerator1" :!type "/Game/Data/ENUM_Weather Enum"))))

(fn `GetTotalSeconds`
  (returns (Seconds :type Integer))
  (bind (_days _hours _minutes _seconds) (`KismetMathLibrary.BreakTimespan` (`self.Time`)))
  (return (+ (* (+ (* _hours 60) _minutes) 60) _seconds)))

(fn `SetLocalTime`
  (set `self.Time` (`KismetMathLibrary.GetTimeOfDay` (`KismetMathLibrary.Now`)))
  (`self.DayCycle`))

(fn `SetTimeUnit`
  (params (CurrentUnit :type Integer) (NextUnit :type Integer) (UnitMax :type Integer))
  (returns (CurrentUnitResult :type Integer) (NextUnitResult :type Integer))
  (if (== CurrentUnit (`local.UnitMax`))
    (`|VariableSetRef` (`local.CurrentUnit`))
    (`/Engine/EditorBlueprintResources/StandardMacros.IncrementInt` (`local.NextUnit`)
      (:`  `
        _)))
  (return (`local.CurrentUnit`) (`local.NextUnit`)))

(fn `SetupDayCycle`
  (bind _returnvalue (`GameplayStatics.GetActorOfClass` "/Game/Blueprints/Misc/BP_LevelLight.BP_LevelLight_C"))
  (bind _output_get (set `self.LevelLighting` _returnvalue))
  (`/Game/Blueprints/Misc/BP_LevelLight.UpdateWeather` _output_get (`self.GetCurrentWeather`))
  (`self.UpdateDay`))

(fn `UpdateDay`
  (bind _levellighting (`self.LevelLighting`)
    (:`then`
      (`/Game/Blueprints/Misc/BP_LevelLight.UpdateDay` _levellighting (`self.GetDayLightAlpha`)))
    (:`else`)))

(fn `UpdateTime`
  (bind (_days _hours _minutes _seconds) (`KismetMathLibrary.BreakTimespan` (`self.Time`)))
  (bind _result (`/Engine/EditorBlueprintResources/StandardMacros.IncrementInt` _seconds)
    (:`  `
      (bind (_currentunitresult _nextunitresult) (`self.SetTimeUnit` _result _minutes 60))
      (bind (_currentunitresult_2 _nextunitresult_2) (`self.SetTimeUnit` _nextunitresult _hours 60))
      (bind (_currentunitresult_3 _nextunitresult_3) (`self.SetTimeUnit` _nextunitresult_2 _days 24))
      (set `self.Time` (`KismetMathLibrary.MakeTimespan` _nextunitresult_3 _currentunitresult_3 _currentunitresult_2 _currentunitresult))
      (`self.UpdateDay`))))