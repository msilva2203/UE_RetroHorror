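; Actor component for Characters that tracks health, stamina and adrenaline and applies fall damage.
; Change functions clamp each stat and broadcast updates; Setup initializes only health and adrenaline.
; When enabled, Tick polls CharacterMovement, using paired DoOnce nodes to catch fall start and landing.
; Landing broadcasts the straight-line 3D fall distance and, beyond a threshold, subtracts health proportional to it.
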(event `self.ReceiveTick`
  (params (DeltaSeconds :type "Float (single-precision)"))
  (if (`self.FallDamageEnabled`)
    (bind _charactermovement (`self.CharacterMovement`)
      (:`then`
        (if (`NavMovementComponent.IsFalling` _charactermovement)
          (`/Engine/EditorBlueprintResources/StandardMacros.DoOnce` true :!label _label
            (:`Completed`
              (`|ExecutionSequence`
                (:`then_0`
                  (set `self.FallStartLocation` (`Actor.K2_GetActorLocation` (`self.GetOwner`)))
                  (set `self.IsFalling` true))
                (:`then_1`
                  (goto _label_2 :!via `Reset`)))))
          (else
            (`/Engine/EditorBlueprintResources/StandardMacros.DoOnce` false :!label _label_2
              (:`Completed`
                (`|ExecutionSequence`
                  (:`then_0`
                    (`self.DealFallDamage`)
                    (set `self.IsFalling` false))
                  (:`then_1`
                    (goto _label :!via `Reset`))))))))
      (:`else`))))

(event `self.ReceiveBeginPlay`
  (`self.Setup`))

(fn `ChangeAdrenaline`
  (params (Offset :type Integer))
  (set `self.Adrenaline` (`KismetMathLibrary.Clamp` (+ Offset (`self.Adrenaline`)) 0 (`self.Max  Adrenaline`)))
  (`self.OnAdrenalineUpdate` (`self.GetAdrenalinePercentage`)))

(fn `ChangeHealth`
  (params (HealthOffset :type Integer))
  (set `self.CurrentHealth` (`KismetMathLibrary.Clamp` (+ (`self.CurrentHealth`) HealthOffset) 0 (`self.MaxHealth`)))
  (`self.OnHealthUpdate` (`self.CurrentHealth`) (`self.GetHealthPercent`) (>= HealthOffset 0)))

(fn `ChangeStamina`
  (params (StaminaOffset :type Integer))
  (set `self.CurrentStamina` (`KismetMathLibrary.Clamp` (+ (`self.CurrentStamina`) StaminaOffset) 0 (`self.MaxStamina`)))
  (`self.OnStaminaUpdate` (`self.CurrentStamina`) (`self.GetStaminaPercent`) (>= StaminaOffset 0)))

(fn `DealFallDamage`
  (bind _returnvalue (`KismetMathLibrary.Vector_Distance` (`Actor.K2_GetActorLocation` (`self.GetOwner`)) (`self.FallStartLocation`)))
  (if (`self.IsFalling`)
    (`self.OnFall` _returnvalue)
    (if (> _returnvalue (`self.MinFallDistance`))
      (`self.ChangeHealth` (* (/ (`KismetMathLibrary.FTrunc` _returnvalue) 100) -1)))))

(fn `GetAdrenalinePercentage`
  (returns (AdrenalinePercentage :type "Float (double-precision)"))
  (return (/ (`KismetMathLibrary.Conv_IntToDouble` (`self.Adrenaline`)) (`KismetMathLibrary.Conv_IntToDouble` (`self.Max  Adrenaline`)))))

(fn `GetHealthPercent`
  (returns (Percent :type "Float (double-precision)"))
  (return (/ (`KismetMathLibrary.Conv_IntToDouble` (`self.CurrentHealth`)) (`KismetMathLibrary.Conv_IntToDouble` (`self.MaxHealth`)))))

(fn `GetStaminaPercent`
  (returns (Percent :type "Float (double-precision)"))
  (return (/ (`KismetMathLibrary.Conv_IntToDouble` (`self.CurrentStamina`)) (`KismetMathLibrary.Conv_IntToDouble` (`self.MaxStamina`)))))

(fn `Kill`
  (`self.ChangeHealth` (* (`self.MaxHealth`) -1)))

(fn `SetFallDamageEnabled`
  (params (Enabled :type Boolean))
  (set `self.FallDamageEnabled` Enabled))

(fn `Setup`
  (bind _ascharacter (cast `Character` (`self.GetOwner`)))
  (set `self.CharacterMovement` (`Character.CharacterMovement` _ascharacter))
  (set `self.CurrentHealth` (`KismetMathLibrary.Clamp` (`self.InitialHealth`) 0 (`self.MaxHealth`)))
  (set `self.Adrenaline` (`KismetMathLibrary.Clamp` (`self.InitialAdrenaline`) 0 (`self.Max  Adrenaline`))))