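; Enemy character that patrols a path, chases visible players, attacks, and can be damaged, pushed or stunned.
; Pawn sensing and player hiding or door events switch BP_AIController between patrol and delayed chase, using cross-resetting DoOnce gates.
; Hiding only restores patrol when the enemy is beyond vulnerability range; attacking a hidden player toggles the hiding spot.
; A timer plays surface-based footsteps, while a proximity-revealed widget shows health with a timeline-lerped trailing bar.
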(event `self.ReceiveBeginPlay`
  (bind _output_get (set `self.AIController` (cast `/Game/Blueprints/BP_AIController` (`AIBlueprintHelperLibrary.GetAIController` self) :!pure true)))
  (set `/Game/Blueprints/BP_AIController.EnemyPawn` self _output_get)
  (`self.InitFoostepTimer`)
  (`self.Patrol`)
  (bind _asbp_player_controller (cast `/Game/Blueprints/BP_PlayerController` (`GameplayStatics.GetPlayerController` 0)))
  (add `/Game/Blueprints/BP_PlayerController.OnPlayerPossessed` _asbp_player_controller (delegate `OnPlayerPossessed`))
  (`self.SetupHealthBar`))

(event `OnPlayerPossessed`
  (params (PlayerCharacter :type "/Game/Blueprints/BP_PlayerCharacter Object Reference"))
  (add `/Game/Blueprints/BP_PlayerCharacter.OnDoorOpen` PlayerCharacter (delegate `OnDoorOpen`))
  (add `/Game/Blueprints/BP_PlayerCharacter.OnPlayerHidden` PlayerCharacter (delegate `OnPlayerHidden`)))

(event `OnDoorOpen`
  (params (Door :type "/Game/Blueprints/BP_Door Object Reference"))
  (`KismetSystemLibrary.PrintString` (`KismetSystemLibrary.GetDisplayName` Door))
  (`self.Patrol`))

(event `OnPlayerHidden`
  (params (IsHidden :type Boolean) (HidingPlace :type "/Game/Blueprints/BP_HidingPlace Object Reference"))
  (if IsHidden
    (bind _output_get (set `self.Hiding Place` HidingPlace))
    (if (`self.IsPlayerVulnerable` _output_get)
      (`KismetSystemLibrary.PrintString` "Player Is Vulnerable in Hiding Spot")
      (else
        (`self.Patrol`)))))

(event `self.BasicCharacterComponent.OnHealthUpdate`
  (params (CurrentHealth :type Integer) (HealthPercent :type "Float (double-precision)") (Positive :type Boolean))
  (`|ExecutionSequence`
    (:`then_0`
      (`GameplayStatics.PlaySound2D` "/Game/SFX/SC_PAIN.SC_PAIN" 1.0 1.0 0.0 null null))
    (:`then_1`
      (if (not (`self.bPlayerInsideRadius`))
        (`/Game/UI/Components/WBP_EnemyBar.PlayDamageAnim` (`self.WBP_EnemyHealth`)))
      (`TimelineComponent.PlayFromStart` (`self.Timeline_Health`)))
    (:`then_2`
      (if (<= CurrentHealth 0)
        (`GameplayStatics.PlaySound2D` "/Game/SFX/SC_DEATH.SC_DEATH" 1.0 1.0 0.0 null null)
        (`self.K2_DestroyActor`)))))

(event `InitFoostepTimer`
  (bind _returnvalue (`KismetSystemLibrary.K2_SetTimerDelegate` (delegate `PlayFootstep`) 0.4 true))
  (set `self.Timer_Footstep` _returnvalue))

(event `PlayFootstep`
  (if (!= (`KismetMathLibrary.VSize` (`self.GetVelocity`)) 0.0)
    (`GameplayStatics.PlaySoundAtLocation` (`self.GetMaterialSound`) (`self.K2_GetActorLocation`) (struct) 1.0 1.0 0.0 null null null null)))

(event `self.PawnSensing.OnSeePawn`
  (params (Pawn :type "Pawn Object Reference"))
  (bind _ishidden (message `/Game/Blueprints/Interfaces/IF_Actions.GetIsHidden` Pawn))
  (if (not _ishidden)
    (`self.Chase` Pawn)))

(event `Patrol`
  (`|ExecutionSequence`
    (:`then_0`
      (`/Engine/EditorBlueprintResources/StandardMacros.DoOnce` false :!label _label
        (:`Completed`
          (bind _newspeed (`self.SetEnemySpeed` (`self.PatrolSpeed`)))
          (`/Game/Blueprints/BP_AIController.Patrol` (`self.AIController`) _newspeed (`self.PatrolPath`))
          (`KismetSystemLibrary.PrintString` "Enemy Is Patroling"))))
    (:`then_1`
      (goto _label_2 :!via `Reset`))))

(event `Chase`
  (params (PlayerPawn :type "Pawn Object Reference"))
  (`|ExecutionSequence`
    (:`then_0`
      (`/Engine/EditorBlueprintResources/StandardMacros.DoOnce` false :!label _label_2
        (:`Completed`
          (`/Game/Blueprints/BP_AIController.StopPatrol` (`self.AIController`))
          (`KismetSystemLibrary.Delay` 3.0)
          (`self.SetEnemySpeed` (`self.ChaseSpeed`))
          (`/Game/Blueprints/BP_AIController.ChasePlayer` (`self.AIController`) PlayerPawn)
          (`KismetSystemLibrary.PrintString` "Enemy Is Chasing"))))
    (:`then_1`
      (goto _label :!via `Reset`))))

(event `self.PawnSensing.OnHearNoise`
  (params (Instigator :type "Pawn Object Reference") (Location :type "Vector Structure (by ref)") (Volume :type "Float (single-precision)"))
  (`KismetSystemLibrary.PrintString` "Sound Heard"))

(event `Attack`
  (params (Pawn :type "Pawn Object Reference"))
  (bind _ishidden (message `/Game/Blueprints/Interfaces/IF_Actions.GetIsHidden` Pawn))
  (if _ishidden
    (`/Game/Blueprints/BP_HidingPlace.ToggleIsHidden` (`self.Hiding Place`))
    (else
      (`/Game/Blueprints/Components/BasicCharacterComponent.OffsetHealth` (`self.GetComponentByClass` Pawn "/Game/Blueprints/Components/BasicCharacterComponent.BasicCharacterComponent_C") (* (`self.EnemyDamage`) -1)))))

(event `/Game/Blueprints/Interfaces/IF_Damage.Damage`
  (params (Damage :type Integer))
  (`/Game/Blueprints/Components/BasicCharacterComponent.OffsetHealth` (`self.BasicCharacterComponent`) (* Damage -1)))

(event `/Game/Blueprints/Interfaces/IF_Damage.Impulse`
  (params (Direction :type "Vector Structure") (Force :type "Float (double-precision)"))
  (`CharacterMovementComponent.AddImpulse` (`self.CharacterMovement`) (* Direction Force) true))

(event `self.OverlapCollision.OnComponentBeginOverlap`
  (params (OverlappedComponent :type "PrimitiveComponent Object Reference") (OtherActor :type "Actor Object Reference") (OtherComp :type "PrimitiveComponent Object Reference") (OtherBodyIndex :type Integer) (bFromSweep :type Boolean) (SweepResult :type "HitResult Structure (by ref)"))
  (bind _wbp_enemyhealth (`self.WBP_EnemyHealth`))
  (if (== OtherActor (`GameplayStatics.GetPlayerPawn` 0))
    (set `self.bPlayerInsideRadius` true)
    (`/Game/UI/Components/WBP_EnemyBar.StopDamageAnim` _wbp_enemyhealth)
    (`/Game/UI/Components/WBP_EnemyBar.SetOpacity` _wbp_enemyhealth 1.0)))

(event `self.OverlapCollision.OnComponentEndOverlap`
  (params (OverlappedComponent :type "PrimitiveComponent Object Reference") (OtherActor :type "Actor Object Reference") (OtherComp :type "PrimitiveComponent Object Reference") (OtherBodyIndex :type Integer))
  (if (== OtherActor (`GameplayStatics.GetPlayerPawn` 0))
    (set `self.bPlayerInsideRadius` false)
    (`/Game/UI/Components/WBP_EnemyBar.SetOpacity` (`self.WBP_EnemyHealth`) 0.0)))

(event `/Game/Blueprints/Interfaces/IF_Damage.Stun`
  (params (StunTime :type "Float (double-precision)"))
  (`/Engine/EditorBlueprintResources/StandardMacros.DoOnce` false :!label _label_3
    (:`Completed`
      (`/Game/Blueprints/BP_AIController.Stop` (`self.AIController`) StunTime (`GameplayStatics.GetPlayerPawn` 0))
      (`KismetSystemLibrary.PrintString` "STUN!!!" true true (struct :`G` 1.0 :`B` 0.012573 :`A` 1.0)))))

(event `EndStun`
  (goto _label_3 :!via `Reset`))

(fn `GetEnemySpeed`
  (returns (Speed :type "Float (single-precision)"))
  (return (`CharacterMovementComponent.MaxWalkSpeed` (`self.CharacterMovement`))))

(fn `GetMaterialSound`
  (returns (ReturnValue :type "SoundCue Object Reference"))
  (bind _returnvalue (`self.K2_GetActorLocation`))
  (bind _outhit (`KismetSystemLibrary.LineTraceSingleForObjects` (+ _returnvalue (0.0 0.0 30.0)) (+ _returnvalue (0.0 0.0 -100.0)) (`|MakeArray` "ObjectTypeQuery1" :!type "EObjectTypeQuery Enum")))
  (return (select `EPhysicalSurface` (`GameplayStatics.GetSurfaceType` _outhit) :`SurfaceType_Default` "/Game/SFX/SC_FS_CONCRETE.SC_FS_CONCRETE" :`SurfaceType1` "/Game/SFX/SC_FS_MUD.SC_FS_MUD" :`SurfaceType2` "/Game/SFX/SC_FS_CONCRETE.SC_FS_CONCRETE" :`SurfaceType3` "/Game/SFX/SC_FS_WATER.SC_FS_WATER" :!type "SoundCue Object Reference")))

(fn `IsPlayerVulnerable`
  (params (HidingPlace :type "/Game/Blueprints/BP_HidingPlace Object Reference"))
  (returns (ReturnValue :type Boolean))
  (return (<= (`KismetMathLibrary.Vector_Distance` (`self.K2_GetActorLocation` HidingPlace) (`self.K2_GetActorLocation`)) (`self.VulnerabilityRange`))))

(fn `SetEnemySpeed`
  (params (Speed :type "Float (double-precision)"))
  (returns (NewSpeed :type "Float (single-precision)"))
  (bind _output_get (set `CharacterMovementComponent.MaxWalkSpeed` Speed (`self.CharacterMovement`)))
  (return _output_get))

(fn `SetupHealthBar`
  (bind _percent (`/Game/Blueprints/Components/BasicCharacterComponent.GetHealthPercent` (`self.BasicCharacterComponent`)))
  (bind _returnvalue (`|CreateWidget` "/Game/UI/Components/WBP_EnemyBar.WBP_EnemyBar_C" (`GameplayStatics.GetPlayerController` 0)))
  (bind _output_get (set `self.WBP_EnemyHealth` _returnvalue))
  (`WidgetComponent.SetWidget` (`self.WC_HealthBar`) _output_get)
  (`/Game/UI/Components/WBP_EnemyBar.SetHealthPercent` (`self.WBP_EnemyHealth`) _percent _percent)
  (set `self.DelayedHealthPercent` _percent))

(fn `UserConstructionScript`)