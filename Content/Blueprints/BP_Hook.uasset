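; BP_Hook is a grapple point that pulls the player character to its capsule's location when Hook is called.
; It locks input and fall damage, plays shake, sound and a timeline that turns the view toward the hook, then moves the player over a time derived from distance and speed.
; HoverArea ignores the Visibility channel during the pull and a short cooldown afterward, with a debug print on each toggle.
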(event `Hook`
  (params (PlayerCharacter :type "/Game/Blueprints/BP_PlayerCharacter Object Reference"))
  (bind _basic_character_component (`/Game/Blueprints/BP_PlayerCharacter.Basic Character Component` PlayerCharacter))
  (`self.SetEnabled` false)
  (`Character.StopJumping` PlayerCharacter)
  (`Character.Jump` PlayerCharacter)
  (`/Game/Blueprints/Components/BasicCharacterComponent.SetFallDamageEnabled` _basic_character_component false)
  (`self.DisableInput` PlayerCharacter (`GameplayStatics.GetPlayerController` 0))
  (`self.HookAnim` PlayerCharacter)
  (`KismetSystemLibrary.Delay` 0.4)
  (`KismetSystemLibrary.MoveComponentTo` (`Character.CapsuleComponent` PlayerCharacter) (`SceneComponent.K2_GetComponentLocation` (`self.Capsule`)) (struct) true false (`self.GetAirTime` (`KismetMathLibrary.Vector_Distance` (`self.K2_GetActorLocation` PlayerCharacter) (`self.K2_GetActorLocation`))))
  (`Character.Jump` PlayerCharacter)
  (`/Game/Blueprints/Components/BasicCharacterComponent.OverrideFalling` _basic_character_component)
  (`self.EnableInput` PlayerCharacter (`GameplayStatics.GetPlayerController` 0))
  (`/Game/Blueprints/Components/BasicCharacterComponent.SetFallDamageEnabled` _basic_character_component true)
  (`KismetSystemLibrary.Delay` 1.5)
  (`self.SetEnabled` true))

(event `HookAnim`
  (params (`Player Character` :type "/Game/Blueprints/BP_PlayerCharacter Object Reference"))
  (bind _returnvalue (`GameplayStatics.GetPlayerController` 0))
  (`PlayerCameraManager.StartCameraShake` :`self` (`GameplayStatics.GetPlayerCameraManager` 0) :`ShakeClass` "/Game/Blueprints/Misc/CShake_Hook.CShake_Hook_C")
  (`GameplayStatics.PlaySoundAtLocation` "/Game/SFX/Files/Interaction/SC_HOOK.SC_HOOK" (`self.K2_GetActorLocation`) (struct) 1.0 1.0 0.0 null null null null)
  (bind (_direction _alpha) (`Timeline|Timeline_Look` :!via `PlayFromStart`)
    (:`Update`
      (`Controller.SetControlRotation` _returnvalue (`KismetMathLibrary.RLerp` (`Controller.GetControlRotation` _returnvalue) (`KismetMathLibrary.FindLookAtRotation` (`self.K2_GetActorLocation` `Player Character`) (`self.K2_GetActorLocation`)) _alpha true)))))

(fn `GetAirTime`
  (params (Distance :type "Float (double-precision)"))
  (returns (Time :type "Float (double-precision)"))
  (return (/ Distance (`self.Speed`))))

(fn `SetEnabled`
  (params (Enabled :type Boolean))
  (`PrimitiveComponent.SetCollisionResponseToChannel` (`self.HoverArea`) "ECC_Visibility" (select `bool` Enabled :`false` "ECR_Ignore" :`true` "ECR_Block" :!type "ECollisionResponse Enum"))
  (`KismetSystemLibrary.PrintString` (`KismetStringLibrary.Conv_BoolToString` Enabled)))

(fn `UserConstructionScript`)