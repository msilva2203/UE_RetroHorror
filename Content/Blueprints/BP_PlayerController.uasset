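; Player controller that owns the HUD and pause menu and tracks gamepad versus keyboard input on the game instance.
; Possessing the player character creates the HUD, shows an opening localized subtitle and broadcasts the possession.
; Helper functions drive prompts, subtitles and tutorials, while pausing swaps the HUD for the menu and switches input mode.
; A debug-style key toggles between a spawned spectator pawn and the character.
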(event `self.ReceiveBeginPlay`
  ;[1 0.7581 0.1451] Begin Play
  (`|ExecutionSequence`
    (:`then_0`
      (bind _asbp_game_instance (cast `/Game/Blueprints/BP_GameInstance` (`GameplayStatics.GetGameInstance`)))
      (bind _output_get (set `self.GameInstance` _asbp_game_instance))
      (`/Game/Blueprints/BP_GameInstance.ChangeInputToGame` _output_get))))

(event `Key|AnyKey` :consume false :paused true
  (params (Key :type "Key Structure"))
  ;[1 0.7581 0.1451] Update Input Device on GameInstance
  (:`Pressed`
    (`/Game/Blueprints/BP_GameInstance.UpdateInputDevice` (`self.GameInstance`) (`KismetInputLibrary.Key_IsGamepadKey` Key))))

(event `InputAction|Pause/Leave`
  (params (Key :type "Key Structure"))
  (:`Pressed`
    (if (not (`self.IsTalking`))
      (`self.SetGamePaused` true))))

(event `Key|+`
  (params (Key :type "Key Structure"))
  (:`Pressed`
    (`/Engine/EditorBlueprintResources/StandardMacros.FlipFlop`
      (:`A`
        (bind _returnvalue (`|SpawnActorFromClass` "/Script/Engine.SpectatorPawn" (`self.GetTransform` (`self.PlayerCharacter`)) "Undefined" "OverrideRootScale" null null))
        (`self.Possess` _returnvalue))
      (:`B`
        (`self.Possess` (`self.PlayerCharacter`))))))

(event `self.ReceivePossess`
  (params (PossessedPawn :type "Pawn Object Reference"))
  (bind _asbp_player_character (cast `/Game/Blueprints/BP_PlayerCharacter` PossessedPawn))
  (set `self.PlayerCharacter` _asbp_player_character)
  (`self.CreateHUD`)
  (`self.ShowSubtitle` (make `/Game/Data/STRUCT_LocalizedText` "Where Am I?" "Onde estou?"))
  (`self.OnPlayerPossessed` (`self.PlayerCharacter`)))

(event `self.ReceiveUnPossess`
  (params (UnpossessedPawn :type "Pawn Object Reference")))

(event `/Game/Blueprints/Interfaces/IF_Actions.SetIsHidden`
  (params (IsHidden :type Boolean) (HidingPlace :type "/Game/Blueprints/BP_HidingPlace Object Reference"))
  (`self.SetHUDVisibility` (select `bool` IsHidden :`false` "Visible" :`true` "Hidden" :!type "ESlateVisibility Enum")))

(event `/Game/Blueprints/Interfaces/IF_Actions.ShowTutorial`
  (params (`Tutorial Text` :type "/Game/Data/STRUCT_LocalizedText Structure") (`Nav Hint` :type "/Game/Data/STRUCT_NavHintSettings Structure"))
  (`/Game/UI/WBP_HUD.ShowTutorial` (`self.GetPlayerHUD`) `Tutorial Text` `Nav Hint` (`/Game/Blueprints/BP_GameInstance.GetLanguage` (`self.GameInstance`))))

(fn `CreateHUD`
  (`/Engine/EditorBlueprintResources/StandardMacros.IsValid` (`self.HUD`)
    (:`Is Valid`
      _)
    (:`Is Not Valid`
      (bind _returnvalue (`|CreateWidget` "/Game/UI/WBP_HUD.WBP_HUD_C" self))
      (set `self.HUD` _returnvalue)))
  (`UserWidget.AddToViewport` (`self.HUD`) 0))

(fn `GetIsHidden`
  (returns (IsHidden :type Boolean))
  (return false))

(fn `GetPlayerHUD`
  (returns (HUD :type "/Game/UI/WBP_HUD Object Reference"))
  (return (`self.HUD`)))

(fn `GetSpeed`
  (returns (Speed :type "Float (double-precision)"))
  (return 0.0))

(fn `HideCrosshair`
  (`/Game/UI/Components/WBP_Crosshair.UpdateCrosshair` :`self` (`/Game/UI/WBP_HUD.WBP_Crosshair` (`self.HUD`))))

(fn `HidePauseMenu`
  (bind _widget_pausemenu (`self.Widget_PauseMenu`)
    (:`then`
      (`Widget.RemoveFromParent` _widget_pausemenu)
      (`WidgetBlueprintLibrary.SetInputMode_GameOnly` self)
      (set `self.bShowMouseCursor` false))
    (:`else`)))

(fn `SetGamePaused`
  (params (Paused :type Boolean))
  (`GameplayStatics.SetGamePaused` Paused)
  (if Paused
    (`self.ShowPauseMenu`)
    (`self.SetHUDVisibility` "Collapsed")
    (else
      (`self.HidePauseMenu`)
      (`self.SetHUDVisibility` "Visible"))))

(fn `SetHUDVisibility`
  (params (InVisibility :type "ESlateVisibility Enum" :default "Visible"))
  (bind _hud (`self.HUD`)
    (:`then`
      (`Widget.SetVisibility` _hud InVisibility))
    (:`else`)))

(fn `ShowPauseMenu`
  (bind _returnvalue (`|CreateWidget` "/Game/UI/Menus/WBP_PauseMenu.WBP_PauseMenu_C" self self))
  (bind _output_get (set `self.Widget_PauseMenu` _returnvalue))
  (`UserWidget.AddToViewport` _output_get 0)
  (`WidgetBlueprintLibrary.SetInputMode_UIOnlyEx` self _output_get)
  (set `self.bShowMouseCursor` true))

(fn `ShowSubtitle`
  (params (Text :type "/Game/Data/STRUCT_LocalizedText Structure") (IsPersistent :type Boolean) (HighlightText :type "/Game/Data/STRUCT_LocalizedText Structure") (HighlightColor :type "LinearColor Structure"))
  (`/Game/UI/Components/WBP_Subtitles.ShowSubtitle` (`/Game/UI/WBP_HUD.WBP_Subtitles` (`self.HUD`)) Text (`/Game/Blueprints/BP_GameInstance.GetLanguage` (`self.GameInstance`)) IsPersistent HighlightText HighlightColor))

(fn `UpdateHUDPrompt`
  (params (NewVisibility :type Boolean) (Hints :type "Array of /Game/Data/STRUCT_NavHintSettings Structure"))
  (`Widget.SetVisibility` (`/Game/UI/WBP_HUD.WBP_NavHintBox` (`self.HUD`)) (select `bool` NewVisibility :`false` "Collapsed" :`true` "Visible" :!type "ESlateVisibility Enum"))
  (if (`local.NewVisibility`)
    (`/Game/UI/Components/WBP_NavHintBox.UpdateBox` (`/Game/UI/WBP_HUD.WBP_NavHintBox` (`self.HUD`)) (`local.Hints`))))

(fn `UserConstructionScript`)