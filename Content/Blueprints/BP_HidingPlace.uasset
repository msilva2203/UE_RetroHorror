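; BP_HidingPlace is an interactable spot where the player hides and looks out through the place's own camera.
; Interacting plays a game instance screen transition, at whose midpoint it swaps view target, sends hidden-state messages and toggles outline custom depth.
; On entry, a child-actor teleporter also moves the player.
; While hidden, clamped look input slows near the angle limits, and the camera eases back to its initial rotation when idle.
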(event `self.ReceiveBeginPlay`
  (`/Game/Blueprints/Components/InteractionComponent.Setup` (`self.InteractionComponent`) (`self.Name`) "NewEnumerator4")
  (bind _asbp_game_instance (cast `/Game/Blueprints/BP_GameInstance` (`GameplayStatics.GetGameInstance`)))
  (set `self.GameInstance` _asbp_game_instance))

(event `InputAxis|LookUp` :consume false
  (params (AxisValue :type "Float (single-precision)"))
  (if (`self.IsHidden`)
    (`self.AddCameraRotation` (* AxisValue -0.1 (`self.GetCameraProximityPercent` (`self.CameraPitch`))))
    (set `self.PitchMoving` (!= AxisValue 0.0))))

(event `/Game/Blueprints/Interfaces/IF_Interaction.OpenInteraction`
  (if (`self.IsActive`)
    (`self.EnableInput` (`GameplayStatics.GetPlayerController` 0))))

(event `InputAxis|Turn` :consume false
  (params (AxisValue :type "Float (single-precision)"))
  (if (`self.IsHidden`)
    (`self.AddCameraRotation` 0.0 (* AxisValue 0.1 (`self.GetCameraProximityPercent` (`self.CameraYaw`))))
    (set `self.YawMoving` (!= AxisValue 0.0))))

(event `/Game/Blueprints/Interfaces/IF_Interaction.CloseInteraction`
  (if (`self.IsActive`)
    (`self.DisableInput` (`GameplayStatics.GetPlayerController` 0))))

(event `self.ReceiveTick`
  (params (DeltaSeconds :type "Float (single-precision)"))
  (bind (_initialrotation_roll _initialrotation_pitch _initialrotation_yaw) (`KismetMathLibrary.BreakRotator` (`self.InitialRotation`)))
  (bind _returnvalue (`KismetMathLibrary.RInterpTo` (`SceneComponent.K2_GetComponentRotation` (`self.ViewCamera`)) (`self.InitialRotation`) DeltaSeconds 5.0))
  (if (and (not (`self.PitchMoving`)) (not (`self.YawMoving`)) (`self.IsHidden`))
    (`SceneComponent.K2_SetWorldRotation` (`self.ViewCamera`) _returnvalue false false)
    (set `self.CameraPitch` (- (.pitch _returnvalue) _initialrotation_pitch))
    (set `self.CameraYaw` (- (.yaw _returnvalue) _initialrotation_yaw))))

(event `InputAction|Interaction`
  (params (Key :type "Key Structure"))
  (:`Pressed`
    (`/Engine/EditorBlueprintResources/StandardMacros.DoOnce` false :!label _label
      (:`Completed`
        (`/Game/Blueprints/BP_GameInstance.PlayTransition` (`self.GameInstance`) (delegate `OnTransitionBegin`) "Forward" 3.5)
        (if (not (`self.IsHidden`))
          (message `/Game/Blueprints/Interfaces/IF_Actions.SetIsHidden` (`GameplayStatics.GetPlayerPawn` 0) true))))))

(event `Reset`
  (goto _label :!via `Reset`))

(event `OnTransitionBegin`
  (bind _returnvalue (`GameplayStatics.GetPlayerController` 0))
  (bind _returnvalue_2 (`GameplayStatics.GetPlayerController` 0))
  (`/Game/Blueprints/BP_GameInstance.PlayTransition` (`self.GameInstance`) (delegate `OnTransitionEnd`) "Reverse" 3.5)
  (`self.Reset`)
  (if (not (`self.IsHidden`))
    (`PlayerController.SetViewTargetWithBlend` _returnvalue self 0.0 "VTBlend_Linear" 0.0 false)
    (message `/Game/Blueprints/Interfaces/IF_Actions.SetIsHidden` _returnvalue true)
    (set `self.IsHidden` true)
    (`/Game/Blueprints/BP_PlayerTeleporter.TeleportPlayer` (cast `/Game/Blueprints/BP_PlayerTeleporter` (`ChildActorComponent.ChildActor` (`self.Teleporter`)) :!pure true) (cast `/Game/Blueprints/BP_PlayerCharacter` (`GameplayStatics.GetPlayerPawn` 0) :!pure true))
    (`PrimitiveComponent.SetRenderCustomDepth` (`self.Mesh`) false)
    (else
      (`PlayerController.SetViewTargetWithBlend` _returnvalue_2 (`GameplayStatics.GetPlayerPawn` 0) 0.0 "VTBlend_Linear" 0.0 false)
      (message `/Game/Blueprints/Interfaces/IF_Actions.SetIsHidden` _returnvalue_2 false)
      (message `/Game/Blueprints/Interfaces/IF_Actions.SetIsHidden` (`GameplayStatics.GetPlayerPawn` 0) false)
      (set `self.IsHidden` false)
      (`self.DisableInput` (`GameplayStatics.GetPlayerController` 0))
      (`PrimitiveComponent.SetRenderCustomDepth` (`self.Mesh`) true))))

(event `OnTransitionEnd`
  (if (`self.IsHidden`)
    (`self.EnableInput` (`GameplayStatics.GetPlayerController` 0))))

(fn `AddCameraRotation`
  (params (Pitch :type "Float (double-precision)") (Yaw :type "Float (double-precision)"))
  (bind (_initialrotation_roll _initialrotation_pitch _initialrotation_yaw) (`KismetMathLibrary.BreakRotator` (`self.InitialRotation`)))
  (bind _max (`self.Max`))
  (bind _returnvalue (* _max -1.0))
  (set `self.CameraPitch` (`KismetMathLibrary.FClamp` (+ Pitch (`self.CameraPitch`)) _returnvalue _max))
  (set `self.CameraYaw` (`KismetMathLibrary.FClamp` (+ Yaw (`self.CameraYaw`)) _returnvalue _max))
  (`SceneComponent.K2_SetWorldRotation` (`self.ViewCamera`) (`KismetMathLibrary.MakeRotator` _initialrotation_roll (+ _initialrotation_pitch (`self.CameraPitch`)) (+ _initialrotation_yaw (`self.CameraYaw`))) false false))

(fn `GetCameraProximityPercent`
  (params (Input :type "Float (double-precision)"))
  (returns (Percent :type "Float (double-precision)"))
  (return (- 1.0005 (/ (`KismetMathLibrary.Abs` Input) (`self.Max`)))))

(fn `SetIsActive`
  (params (NewIsActive :type Boolean))
  (bind _output_get (set `self.IsActive` NewIsActive))
  (`PrimitiveComponent.SetRenderCustomDepth` (`self.Mesh`) _output_get))

(fn `UserConstructionScript`
  (`self.SetIsActive` (`self.IsActive`))
  (set `self.InitialRotation` (`SceneComponent.K2_GetComponentRotation` (`self.ViewCamera`))))