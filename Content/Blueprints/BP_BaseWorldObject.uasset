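; Base Blueprint for world objects whose state is stored in BP_GameInstance: tutorials, doors, telephones and pickups.
; On BeginPlay it caches the game instance, reads its state from the array chosen by StateType at ObjectIndex, and passes it to SetupObject, an empty event here.
; SetWorldState writes a new state back through the game instance's UpdateWorldState and prints a confirmation.
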(event `self.ReceiveBeginPlay`
  (bind _asbp_game_instance (cast `/Game/Blueprints/BP_GameInstance` (`GameplayStatics.GetGameInstance`)))
  (set `self.GameInstance` _asbp_game_instance)
  (`self.SetupObject` (`self.GetWorldState`)))

(event `SetupObject`
  (params (State :type Boolean)))

(fn `GetWorldState`
  (returns (State :type Boolean))
  (bind (_statetutorials _statedoors _statetelephones _statepickups) (break `/Game/Data/STRUCT_WorldState` (`/Game/Blueprints/BP_GameInstance.GetWorldStateData` (`self.GameInstance`))))
  (return (`|GetArrayItem` (select `/Game/Data/ENUM_WorldStateType` (`self.StateType`) :`NewEnumerator0` _statetutorials :`NewEnumerator1` _statedoors :`NewEnumerator2` _statetelephones :`NewEnumerator3` _statepickups) (`self.ObjectIndex`))))

(fn `SetWorldState`
  (params (State :type Boolean))
  (locals (TempStates :type "Array of Boolean"))
  (`/Game/Blueprints/BP_GameInstance.UpdateWorldState` (`self.GameInstance`) (`self.StateType`) (`self.ObjectIndex`) State)
  (`KismetSystemLibrary.PrintString` "World State Updated successfully"))

(fn `UserConstructionScript`)