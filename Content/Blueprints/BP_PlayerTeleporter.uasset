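; BP_PlayerTeleporter is a placeable point that either moves an existing player to itself or spawns a new player character there.
; A downward visibility trace from its LocationArrow finds the destination, falling back to the arrow's position when nothing is hit.
; Teleporting moves the player and matches control rotation to the arrow.
; Spawning creates a BP_PlayerCharacter facing the arrow, restores its saved inventory and possesses it with the first player controller.
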(fn `GetSpawnLocation`
  (returns (Location :type "Vector Structure"))
  (bind _returnvalue (`SceneComponent.K2_GetComponentLocation` (`self.LocationArrow`)))
  (bind (_outhit _returnvalue_2) (`KismetSystemLibrary.LineTraceSingle` _returnvalue (+ _returnvalue (0.0 0.0 -2000.0)) "TraceTypeQuery1"))
  (if _returnvalue_2
    (return (`.Location` (`GameplayStatics.BreakHitResult` _outhit)))
    (else
      (return (`SceneComponent.K2_GetComponentLocation` (`self.LocationArrow`))))))

(fn `SpawnPlayer`
  (params (SavedInventory :type "Array of /Game/Data/STRUCT_InventoryItem Structure"))
  (bind _returnvalue (`|SpawnActorFromClass` "/Game/Blueprints/BP_PlayerCharacter.BP_PlayerCharacter_C" (`KismetMathLibrary.MakeTransform` (`self.GetSpawnLocation`) (`SceneComponent.K2_GetComponentRotation` (`self.LocationArrow`))) "AlwaysSpawn" "OverrideRootScale" null null))
  (`/Game/Blueprints/BP_PlayerCharacter.RetrieveSavedData` _returnvalue (`local.SavedInventory`))
  (`Controller.Possess` (`GameplayStatics.GetPlayerController` 0) _returnvalue))

(fn `TeleportPlayer`
  (params (Player :type "/Game/Blueprints/BP_PlayerCharacter Object Reference"))
  (`self.K2_SetActorLocation` Player (`self.GetSpawnLocation`) false false)
  (`Controller.SetControlRotation` (`GameplayStatics.GetPlayerController` 0) (`SceneComponent.K2_GetComponentRotation` (`self.LocationArrow`))))

(fn `UserConstructionScript`)