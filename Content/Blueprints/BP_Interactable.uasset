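; BP_Interactable is a pickup actor that adds its item to the player's inventory with a short camera showcase.
; The construction script loads the item from DT_GameItems by clamped index and sets both meshes, overlaying M_Interactable on the extra one.
; Open and close events toggle its input.
; Interacting adds the item, switches view to the slowly rotating camera arm, hides the pawn, then after a delay restores the player and destroys itself.
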(event `self.ReceiveTick`
  (params (DeltaSeconds :type "Float (single-precision)"))
  (if (`self.IsOpen`)
    (`SceneComponent.K2_AddRelativeRotation` (`self.CameraArm`) (struct :`Yaw` 0.5) false false)))

(event `/Game/Blueprints/Interfaces/IF_Interaction.OpenInteraction`
  (`self.EnableInput` (`GameplayStatics.GetPlayerController` 0)))

(event `/Game/Blueprints/Interfaces/IF_Interaction.CloseInteraction`
  (`self.DisableInput` (`GameplayStatics.GetPlayerController` 0)))

(event `InputAction|Interaction`
  (params (Key :type "Key Structure"))
  (bind _returnvalue (`GameplayStatics.GetPlayerController` 0))
  (:`Pressed`
    (`/Game/Blueprints/Components/InventoryComponent.AddToInventory` (`self.GetComponentByClass` (`Controller.K2_GetPawn` (`GameplayStatics.GetPlayerController` 0)) "/Game/Blueprints/Components/InventoryComponent.InventoryComponent_C") (`self.Item`))
    (`PlayerController.SetViewTargetWithBlend` (`GameplayStatics.GetPlayerController` 0) self 0.0 "VTBlend_Linear" 0.0 false)
    (`self.SetPlayerHidden` true)
    (set `self.IsOpen` true)
    (`KismetSystemLibrary.Delay` 3.0)
    (`PlayerController.SetViewTargetWithBlend` _returnvalue (`Controller.K2_GetPawn` _returnvalue) 0.5 "VTBlend_Linear" 0.0 false)
    (`self.SetPlayerHidden` false)
    (set `self.IsOpen` false)
    (`self.K2_DestroyActor`)))

(event `self.ReceiveBeginPlay`)

(fn `FindFromDataTable`
  (bind _returnvalue (`KismetMathLibrary.Clamp` (`self.ItemIndex`) 0 (- (`KismetArrayLibrary.Array_Length` (`self.ItemNames`)) 1)))
  (bind _outrownames (`DataTableFunctionLibrary.GetDataTableRowNames` "/Game/Data/DT_GameItems.DT_GameItems"))
  (bind _output_get (set `self.ItemNames` _outrownames))
  (bind _returnvalue_2 (`|GetDataTableRow` "/Game/Data/DT_GameItems.DT_GameItems" (`|GetArrayItem` _output_get _returnvalue))
    (:`then`
      (bind _output_get_2 (set `self.Item` _returnvalue_2))
      (set `self.ItemIndex` _returnvalue)
      (`|VariableSetRef` (`.Quantity_20_29F77E864F14E7BEB05B07BC98EBCE1E` (break `/Game/Data/STRUCT_InventoryItem` _output_get_2)) (`self.Quantity`)))))

(fn `SetPlayerHidden`
  (params (bNewHidden :type Boolean))
  (bind _returnvalue (`GameplayStatics.GetPlayerController` 0))
  (bind _returnvalue_2 (`Controller.K2_GetPawn` _returnvalue))
  (`self.SetActorHiddenInGame` _returnvalue_2 bNewHidden)
  (if (`local.bNewHidden`)
    (`self.DisableInput` _returnvalue_2 _returnvalue)
    (else
      (`self.EnableInput` _returnvalue_2 _returnvalue))))

(fn `UserConstructionScript`
  (bind _mesh (`self.GetMesh`))
  (`self.FindFromDataTable`)
  (`StaticMeshComponent.SetStaticMesh` (`self.StaticMesh`) _mesh)
  (`StaticMeshComponent.SetStaticMesh` (`self.ExtraMesh`) _mesh)
  (`PrimitiveComponent.SetMaterial` (`self.ExtraMesh`) 0 "/Game/Materials/M_Interactable.M_Interactable"))