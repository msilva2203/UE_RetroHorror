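; Interactable NPC actor that turns toward the player and plays linear subtitle dialogue.
; An interaction component handles setup and crosshair, while open/close events toggle the NPC's input.
; Interacting disables pawn input, shows nav hints and runs a yaw-only look-at timeline, whose forward finish starts the dialogue.
; Next advances lines; leaving or running out reverses the turn, restores pawn input and shows a farewell subtitle.
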(event `self.ReceiveBeginPlay`
  (set `self.InitialRotation` (`self.K2_GetActorRotation`))
  (bind _asbp_player_controller (cast `/Game/Blueprints/BP_PlayerController` (`GameplayStatics.GetPlayerController` 0)))
  (set `self.PlayerController` _asbp_player_controller)
  (`/Game/Blueprints/Components/InteractionComponent.Setup` (`self.InteractionComponent`) (`self.Name`) "NewEnumerator2"))

(event `/Game/Blueprints/Interfaces/IF_Interaction.OpenInteraction`
  (`self.EnableInput` (`GameplayStatics.GetPlayerController` 0)))

(event `/Game/Blueprints/Interfaces/IF_Interaction.CloseInteraction`
  (`self.DisableInput` (`GameplayStatics.GetPlayerController` 0)))

(event `InputAction|Interaction`
  (params (Key :type "Key Structure"))
  (:`Pressed`
    (`self.SetLookingAt` true)
    (`self.DisableInput` (`GameplayStatics.GetPlayerPawn` 0) (`GameplayStatics.GetPlayerController` 0))
    (`/Game/Blueprints/Components/InteractionComponent.UpdateCrosshair` (`self.InteractionComponent`) false)
    (`/Game/UI/WBP_HUD.UpdateNavHintBox` (`/Game/Blueprints/BP_PlayerController.GetPlayerHUD` (`self.PlayerController`)) (`self.NavHints`) "NewEnumerator0")
    (`self.SetIsTalking` true)))

(event `InputAction|Pause/Leave`
  (params (Key :type "Key Structure"))
  (:`Pressed`
    (if (`self.IsTalking`)
      (`self.Leave`))))

(event `InputAction|Next`
  (params (Key :type "Key Structure"))
  (:`Pressed`
    (if (`self.IsTalking`)
      (`self.ShowDialogue` (+ (`self.Index`) 1)))))

(event `SetLookingAt`
  (params (IsLooking :type Boolean))
  (if IsLooking
    (bind (_direction _alpha) (`Timeline|Timeline_LookAt` :!label _label)
      (:`Update`
        (`self.K2_SetActorRotation` (`KismetMathLibrary.RLerp` (`self.InitialRotation`) (`self.GetLookAtRotation`) _alpha true)))
      (:`Finished`
        (switch `ETimelineDirection` _direction
          (:`Forward`
            (`self.ShowDialogue` 0)))))
    (else
      (goto _label :!via `Reverse`))))

(fn `GetCurrentDialogue`
  (returns (Output :type "/Game/Data/STRUCT_LocalizedText Structure"))
  (return (`|GetArrayItem` (`self.Dialogue`) (`self.Index`))))

(fn `GetGameInstance`
  (returns (GameInstance :type "/Game/Blueprints/BP_GameInstance Object Reference"))
  (return (`/Game/Blueprints/BP_PlayerController.GameInstance` (`self.PlayerController`))))

(fn `GetLanguage`
  (returns (Language :type "/Game/Data/ENUM_Language Enum"))
  (return (`/Game/Blueprints/BP_GameInstance.GetLanguage` (`self.GetGameInstance`))))

(fn `GetLookAtRotation`
  (returns (Rotation :type "Rotator Structure"))
  (bind (_initialrotation_roll _initialrotation_pitch) (`KismetMathLibrary.BreakRotator` (`self.InitialRotation`)))
  (bind (_returnvalue_roll _returnvalue_pitch _returnvalue_yaw) (`KismetMathLibrary.BreakRotator` (`KismetMathLibrary.FindLookAtRotation` (`self.K2_GetActorLocation`) (`self.K2_GetActorLocation` (`GameplayStatics.GetPlayerPawn` 0)))))
  (return (`KismetMathLibrary.MakeRotator` _initialrotation_roll _initialrotation_pitch _returnvalue_yaw)))

(fn `Leave`
  (bind _hud (`/Game/Blueprints/BP_PlayerController.GetPlayerHUD` (`self.PlayerController`)))
  (`self.SetLookingAt` false)
  (`self.SetIsTalking` false)
  (`self.EnableInput` (`GameplayStatics.GetPlayerPawn` 0) (`GameplayStatics.GetPlayerController` 0))
  (`/Game/UI/WBP_HUD.ClearNavHintBox` _hud)
  (`/Game/UI/WBP_HUD.ShowSubtitle` _hud (`self.LeaveDialogue`) (`self.GetLanguage`) false))

(fn `SetIsTalking`
  (params (NewValue :type Boolean))
  (bind _output_get (set `self.IsTalking` NewValue))
  (set `/Game/Blueprints/BP_PlayerController.IsTalking` _output_get (`self.PlayerController`)))

(fn `ShowDialogue`
  (params (NewIndex :type Integer))
  (bind _output_get (set `self.Index` NewIndex))
  (if (<= _output_get (- (`KismetArrayLibrary.Array_Length` (`self.Dialogue`)) 1))
    (`/Game/Blueprints/BP_PlayerController.ShowSubtitle` (`self.PlayerController`) (`self.GetCurrentDialogue`) true)
    (else
      (`self.Leave`))))

(fn `UserConstructionScript`)