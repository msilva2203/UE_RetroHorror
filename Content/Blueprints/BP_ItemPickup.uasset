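; World item pickup that adds its item and quantity to the interacting pawn's InventoryComponent and shows a localized pickup subtitle.
; The construction script looks up the Item enum in DT_GameItems to set the name, then sets up the mesh and InteractionComponent.
; On interaction, a NETALL event disables collision and plays a timeline meant to pull the mesh toward the pawn before server-side destruction.
; SetupObject destroys the actor when passed a true state.
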(event `self.ReceiveBeginPlay`
  (`parent.ReceiveBeginPlay`)
  (bind _asbp_player_controller (cast `/Game/Blueprints/BP_PlayerController` (`GameplayStatics.GetPlayerController` 0)))
  (set `self.PlayerController` _asbp_player_controller)
  (`TimelineComponent.SetPlayRate` (`self.Timeline_Pickup`) (`self.PickupPlayRate`)))

(event `self.SetupObject`
  (params (State :type Boolean))
  (if State
    (`self.K2_DestroyActor`)))

(event `/Game/Blueprints/Interfaces/IF_Interaction.OpenInteraction`
  (params (PlayerController :type "PlayerController Object Reference"))
  (`self.EnableInput` PlayerController))

(event `/Game/Blueprints/Interfaces/IF_Interaction.CloseInteraction`
  (params (PlayerController :type "PlayerController Object Reference"))
  (`self.DisableInput` PlayerController))

(event `InputAction|Interaction`
  (params (Key :type "Key Structure"))
  (:`Pressed`
    (`/Engine/EditorBlueprintResources/StandardMacros.DoOnce` false
      (:`Completed`
        (message `/Game/Blueprints/Interfaces/IF_Interaction.Interact` (`GameplayStatics.GetPlayerController` 0) self null false false)))))

(event `/Game/Blueprints/Interfaces/IF_Interaction.Interact`
  (params (Actor :type "Actor Object Reference") (PlayerController :type "PlayerController Object Reference") (IsLocked :type Boolean) (DidOpenInventory :type Boolean))
  (bind _returnvalue (`Controller.K2_GetPawn` PlayerController))
  (`/Game/Blueprints/Components/InventoryComponent.AddToInventory` (`self.GetComponentByClass` _returnvalue "/Game/Blueprints/Components/InventoryComponent.InventoryComponent_C") (`self.Item`) (`self.Quantity`))
  (message `/Game/Blueprints/Interfaces/IF_Actions.ShowSubtitleAction` PlayerController (make `/Game/Data/STRUCT_LocalizedText` "You Picked Up " "Tu Apanhas-te ") false (`self.ItemName`) (struct :`G` 1.0 :`B` 0.012573 :`A` 1.0))
  (`self.NETALL_OnPickup` _returnvalue))

(event `NETALL_OnPickup`
  (params (Actor :type "Actor Object Reference"))
  (set `self.AnimTargetActor` Actor)
  (`PrimitiveComponent.SetCollisionEnabled` (`self.StaticMesh`) "NoCollision")
  (`TimelineComponent.Play` (`self.Timeline_Pickup`)))

(fn `FindFromDataTable`
  (bind _returnvalue (`|GetDataTableRow` "/Game/Data/DT_GameItems.DT_GameItems" (`KismetStringLibrary.Conv_StringToName` (`|GetEnumeratorNameAsString` (`self.Item`))))
    (:`then`
      (bind _output_get (set `self.ItemSample` _returnvalue))
      (bind (_item _quantity _itemname) (break `/Game/Data/STRUCT_InventoryItem` _output_get))
      (`|VariableSetRef` _quantity (`self.Quantity`))
      (set `self.ItemName` _itemname))))

(fn `GetPickupLocation`
  (returns (Location :type "Vector Structure"))
  (return (`KismetMathLibrary.MakeVector` (.x (`self.K2_GetActorLocation` (`GameplayStatics.GetPlayerPawn` 0))) (.y (`self.K2_GetActorLocation` (`GameplayStatics.GetPlayerPawn` 0))) (- (.z (`self.K2_GetActorLocation` (`GameplayStatics.GetPlayerPawn` 0))) 30.0))))

(fn `UserConstructionScript`
  (`self.FindFromDataTable`)
  (`StaticMeshComponent.SetStaticMesh` (`self.StaticMesh`) (`self.GetMesh`))
  (`/Game/Blueprints/Components/InteractionComponent.Setup` (`self.InteractionComponent`) (`.ItemName_28_86FAA0354115127B5271D291B2D32D79` (break `/Game/Data/STRUCT_InventoryItem` (`self.ItemSample`))) "NewEnumerator0"))