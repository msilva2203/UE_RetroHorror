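; Interactable item base that can be locked behind a key item from the player's inventory, with empty OnInteraction and Unlock hook events.
; Opening or closing interaction toggles input; the interact key fires OnInteraction and, when locked, opens a filtered inventory.
; Using an item closes the inventory and passes the key match to Unlock.
; A second binding, removed on inventory close, fires unlocked OnInteraction when KeyItem's value is zero.
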(event `self.ReceiveBeginPlay`
  (`parent.ReceiveBeginPlay`)
  (`/Game/Blueprints/Components/InteractionComponent.Setup` (`self.InteractionComponent`) (`self.Name`) "NewEnumerator1")
  (bind _asbp_player_controller (cast `/Game/Blueprints/BP_PlayerController` (`GameplayStatics.GetPlayerController` 0)))
  (set `self.PlayerController` _asbp_player_controller))

(event `/Game/Blueprints/Interfaces/IF_Interaction.OpenInteraction`
  (`self.EnableInput` (`self.PlayerController`)))

(event `/Game/Blueprints/Interfaces/IF_Interaction.CloseInteraction`
  (`self.DisableInput` (`self.PlayerController`)))

(event `InputAction|Interaction`
  (params (Key :type "Key Structure"))
  (bind _returnvalue (`self.GetPlayerInventory`))
  (:`Pressed`
    (`self.OnInteraction` (`self.IsLocked`))
    (if (`self.IsLocked`)
      (`/Game/Blueprints/Components/InventoryComponent.OpenInventory` _returnvalue "NewEnumerator1" (delegate `ItemUsed`))
      (add `/Game/Blueprints/Components/InventoryComponent.OnItemUsed` _returnvalue (delegate `OnItemUsed`))
      (add `/Game/Blueprints/Components/InventoryComponent.OnInventoryClose` (`self.GetPlayerInventory`) (delegate `OnIventoryClose`)))))

(event `OnItemUsed`
  (params (Item :type "/Game/Data/STRUCT_InventoryItem Structure"))
  (if (== 0 (`KismetMathLibrary.Conv_ByteToInt` (`self.KeyItem`)))
    (`self.OnInteraction` false)))

(event `OnIventoryClose`
  (remove `/Game/Blueprints/Components/InventoryComponent.OnItemUsed` (`self.GetPlayerInventory`) (delegate `OnItemUsed`)))

(event `ItemUsed`
  (params (Item :type "/Game/Data/STRUCT_InventoryItem Structure") (CurrentInventory :type "/Game/Blueprints/BP_Inventory Object Reference"))
  (`/Game/Blueprints/BP_Inventory.Close` CurrentInventory)
  (`self.Unlock` (`|EnumEquality` (`.Item_27_04A9D5AC4AACCB80CE078FADF073EE6A` (break `/Game/Data/STRUCT_InventoryItem` Item)) (`self.KeyItem`))))

(event `Unlock`
  (params (Unlock :type Boolean :default true)))

(event `OnInteraction`
  (params (IsLocked :type Boolean)))

(fn `GetPlayerInventory`
  (returns (ReturnValue :type "/Game/Blueprints/Components/InventoryComponent Object Reference"))
  (return (`self.GetComponentByClass` (`GameplayStatics.GetPlayerPawn` 0) "/Game/Blueprints/Components/InventoryComponent.InventoryComponent_C")))

(fn `UserConstructionScript`)