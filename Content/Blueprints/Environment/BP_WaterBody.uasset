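; BP_WaterBody is a box-shaped water volume that notifies entering actors and kills characters that reach its death layer.
; The construction script sizes two boxes from shared X/Y extents, with DeathCollision thinner than Collision.
; Collision sets each actor's environment body state on enter and exit, splashing for non-WorldStatic components.
; DeathCollision calls Kill on any BasicCharacterComponent, armed only after a short delay from BeginPlay.
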(event `self.ReceiveBeginPlay`
  (`KismetSystemLibrary.Delay` 2.0)
  (set `self.CanKill` true))

(event `self.Collision.OnComponentBeginOverlap`
  (params (OverlappedComponent :type "PrimitiveComponent Object Reference") (OtherActor :type "Actor Object Reference") (OtherComp :type "PrimitiveComponent Object Reference") (OtherBodyIndex :type Integer) (bFromSweep :type Boolean) (SweepResult :type "HitResult Structure (by ref)"))
  (message `/Game/Blueprints/Interfaces/IF_Actions.SetActorEnvironmentBody` OtherActor "NewEnumerator1")
  (if (`|EnumInequality` (`PrimitiveComponent.GetCollisionObjectType` OtherComp) "ECC_WorldStatic")
    (`GameplayStatics.PlaySoundAtLocation` "/Game/SFX/Physics/SC_WATER_SPLASH.SC_WATER_SPLASH" (`SceneComponent.K2_GetComponentLocation` OtherComp) (struct) 1.0 1.0 0.0 null null null null)
    (`KismetSystemLibrary.PrintString` "Water body!!" true true (struct :`G` 0.168437 :`B` 0.255208 :`A` 1.0))))

(event `self.Collision.OnComponentEndOverlap`
  (params (OverlappedComponent :type "PrimitiveComponent Object Reference") (OtherActor :type "Actor Object Reference") (OtherComp :type "PrimitiveComponent Object Reference") (OtherBodyIndex :type Integer))
  (message `/Game/Blueprints/Interfaces/IF_Actions.SetActorEnvironmentBody` OtherActor "NewEnumerator0"))

(event `self.DeathCollision.OnComponentBeginOverlap`
  (params (OverlappedComponent :type "PrimitiveComponent Object Reference") (OtherActor :type "Actor Object Reference") (OtherComp :type "PrimitiveComponent Object Reference") (OtherBodyIndex :type Integer) (bFromSweep :type Boolean) (SweepResult :type "HitResult Structure (by ref)"))
  (bind _returnvalue (`self.GetComponentByClass` OtherActor "/Game/Blueprints/Components/BasicCharacterComponent.BasicCharacterComponent_C"))
  (if (`self.CanKill`)
    (`/Engine/EditorBlueprintResources/StandardMacros.IsValid` _returnvalue
      (:`Is Valid`
        (`/Game/Blueprints/Components/BasicCharacterComponent.Kill` _returnvalue)
        (`KismetSystemLibrary.PrintString` "WATER KILLED THE PLAYER")))))

(fn `UserConstructionScript`
  (`BoxComponent.SetBoxExtent` (`self.Collision`) (`KismetMathLibrary.MakeVector` (`self.BoxExtentX`) (`self.BoxExtentY`) 20.0) true)
  (`BoxComponent.SetBoxExtent` (`self.DeathCollision`) (`KismetMathLibrary.MakeVector` (`self.BoxExtentX`) (`self.BoxExtentY`) 5.0) true)
  (`KismetSystemLibrary.PrintString` "Water Setup"))