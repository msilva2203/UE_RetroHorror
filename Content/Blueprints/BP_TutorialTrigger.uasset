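; BP_TutorialTrigger is a trigger volume that shows a tutorial message the first time a player-controlled pawn overlaps it.
; On setup, if its state is not already set, it loads text and nav hint from DT_Tutorials, using the Tutorial enum as row name.
; On overlap it sends them to the first player controller and sets its world state, blocking repeat displays.
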(event `self.SetupObject`
  (params (State :type Boolean))
  (if (not State)
    (`self.RetrieveData`)))

(event `self.Trigger.OnComponentBeginOverlap`
  (params (OverlappedComponent :type "PrimitiveComponent Object Reference") (OtherActor :type "Actor Object Reference") (OtherComp :type "PrimitiveComponent Object Reference") (OtherBodyIndex :type Integer) (bFromSweep :type Boolean) (SweepResult :type "HitResult Structure (by ref)"))
  (bind _aspawn (cast `Pawn` OtherActor))
  (if (and (`Pawn.IsPlayerControlled` _aspawn) (not (`self.GetWorldState`)))
    (`self.ShowTutorial`)))

(fn `RetrieveData`
  (bind _returnvalue (`|GetDataTableRow` "/Game/Data/DT_Tutorials.DT_Tutorials" (`KismetStringLibrary.Conv_StringToName` (`|GetEnumeratorNameAsString` (`self.Tutorial`))))
    (:`then`
      (set `self.TutorialInfo` _returnvalue))))

(fn `ShowTutorial`
  (bind (_tutorialtext _navhint) (break `/Game/Data/STRUCT_Tutorial` (`self.TutorialInfo`)))
  (message `/Game/Blueprints/Interfaces/IF_Actions.ShowTutorial` (`GameplayStatics.GetPlayerController` 0) _tutorialtext _navhint)
  (`self.SetWorldState` true)
  (`KismetSystemLibrary.PrintString` "Tutorial Shown"))

(fn `UserConstructionScript`)