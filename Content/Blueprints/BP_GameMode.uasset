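; Game mode that handles streamed level transitions through tagged doors and caches the BP_PlayerController on login.
; TransitionLevels unloads the current level, loads the next, then ends the transition on the BP_Door matching the transition tag.
; If no door matches, it calls itself with the levels swapped to reverse the move.
; The day-cycle clock is unfinished: StartDayCicle is empty and its one-second timer logic is disconnected.
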(event `self.ReceiveBeginPlay`
  (`self.StartDayCicle`))

(event `self.K2_PostLogin`
  (params (NewPlayer :type "PlayerController Object Reference"))
  (bind _asbp_player_controller (cast `/Game/Blueprints/BP_PlayerController` NewPlayer))
  (set `self.PlayerController` _asbp_player_controller))

(event `SetupVisualOptions`)

(event `StartDayCicle`)

(event `UpdateDayCicle`
  (bind (_year _month _day _hour _minute _second) (`KismetMathLibrary.BreakDateTime` (`self.Time`)))
  (bind _result (`/Engine/EditorBlueprintResources/StandardMacros.IncrementInt` _second)
    (:`  `
      (`self.UpdateTime` _hour _minute _result))))

(event `TransitionLevels`
  (params (CurrentWorld :type "World Soft Object Reference") (NextWorld :type "World Soft Object Reference") (TransitionData :type "/Game/Data/STRUCT_TransitionData Structure"))
  (bind (_playercharacter _transitionwidget _transitiontag) (break `/Game/Data/STRUCT_TransitionData` TransitionData))
  (bind (_door _found) (`self.GetDoorWithTag` _transitiontag))
  ;[1 0.7581 0.1451] Level Loading
  (`GameplayStatics.UnloadStreamLevelBySoftObjectPtr` CurrentWorld)
  (`GameplayStatics.LoadStreamLevelBySoftObjectPtr` NextWorld true)
  (if _found
    (`/Game/Blueprints/BP_Door.EndTransition` _door _playercharacter _transitionwidget (`/Game/Blueprints/BP_Door.GetSelfTeleporter` _door))
    (else
      (`self.TransitionLevels` NextWorld CurrentWorld (make `/Game/Data/STRUCT_TransitionData` _playercharacter _transitionwidget _transitiontag)))))

(fn `GetDoorWithTag`
  (params (Tag :type Text))
  (returns (Door :type "/Game/Blueprints/BP_Door Object Reference") (Found :type Boolean))
  (locals (TempDoor :type "/Game/Blueprints/BP_Door Object Reference") (TempFound :type Boolean))
  (bind _outactors (`GameplayStatics.GetAllActorsOfClass` "/Game/Blueprints/BP_Door.BP_Door_C"))
  (for _array_element _outactors
    (if (== (`/Game/Blueprints/BP_Door.GetTag` _array_element) (`local.Tag`))
      (set `local.TempDoor` _array_element)
      (set `local.TempFound` true)
      (break)))
  (return (`local.TempDoor`) (`local.TempFound`)))

(fn `UpdateTime`
  (params (Hour :type Integer) (Minute :type Integer) (Seconds :type Integer))
  (set `self.Time` (`KismetMathLibrary.MakeDateTime` 0 0 0 Hour Minute Seconds)))

(fn `UserConstructionScript`)