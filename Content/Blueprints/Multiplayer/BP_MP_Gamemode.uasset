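; Multiplayer game mode that tracks joining player controllers and handles the match start and batched respawns.
; A short start timer, cleared on login and restarted once a new player is handled, spawns everyone and begins a looping timer that respawns queued controllers.
; Spawning replaces each possessed pawn with a new character at an index-matched PlayerStart, changes client mode, then notifies all players of new pawns after a short delay.
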(event `self.ReceiveBeginPlay`
  (`self.InitStartTimer`))

(event `self.K2_PostLogin`
  (params (NewPlayer :type "PlayerController Object Reference"))
  (bind _asbp_mp_player_controller (cast `/Game/Blueprints/Multiplayer/BP_MP_PlayerController` NewPlayer))
  (`KismetArrayLibrary.Array_Add` (`self.Players`) _asbp_mp_player_controller)
  (`self.StopStartTimer`))

(event `self.HandleStartingNewPlayer`
  (params (NewPlayer :type "PlayerController Object Reference"))
  (if (`KismetArrayLibrary.Array_Contains` (`self.Players`) (cast `/Game/Blueprints/Multiplayer/BP_MP_PlayerController` NewPlayer :!pure true))
    (`self.InitStartTimer`)))

(event `InitStartTimer`
  ;[1 0.7581 0.1451 1 30] Start Timer
  (bind _returnvalue (`KismetSystemLibrary.K2_SetTimerDelegate` (delegate `OnGameStart`) 2.0))
  (set `self.Timer_Start` _returnvalue))

(event `OnGameStart`
  ;[1 0.7581 0.1451 1 30] Start Timer
  (`self.SpawnPlayers` (`self.Players`))
  (`self.InitRespawnTimer` 5.0))

(event `StopStartTimer`
  ;[1 0.7581 0.1451 1 30] Start Timer
  (`KismetSystemLibrary.K2_ClearAndInvalidateTimerHandle` (`self.Timer_Start`)))

(event `InitRespawnTimer`
  (params (Time :type "Float (double-precision)"))
  ;[1 0.7581 0.1451 1 30] Respawn Timer
  (bind _returnvalue (`KismetSystemLibrary.K2_SetTimerDelegate` (delegate `OnRespawn`) Time true))
  (set `self.Timer_Respawn` _returnvalue))

(event `OnRespawn`
  (bind _spawnwaitingplayers (`self.SpawnWaitingPlayers`))
  ;[1 0.7581 0.1451 1 30] Respawn Timer
  (if (`KismetArrayLibrary.Array_IsNotEmpty` _spawnwaitingplayers)
    (`self.SpawnPlayers` _spawnwaitingplayers)
    (`KismetArrayLibrary.Array_Clear` (`self.SpawnWaitingPlayers`))))

(event `StopRespawnTimer`
  ;[1 0.7581 0.1451 1 30] Respawn Timer
  (`KismetSystemLibrary.K2_ClearAndInvalidateTimerHandle` (`self.Timer_Respawn`)))

(event `NotifyPawnSpawn`
  (params (Pawns :type "Array of /Game/Blueprints/Multiplayer/BP_MP_PlayerCharacter Object Reference (by ref)"))
  ;[1 0.7581 0.1451 1 30] Notify Pawn Spawn to all players
  (`KismetSystemLibrary.Delay` 0.5)
  (for _array_element (`self.Players`)
    (`/Game/Blueprints/Multiplayer/BP_MP_PlayerController.CLIENT Event Pawns Spawn` _array_element Pawns)))

(fn `AddControllerToSpawnList`
  (params (Controller :type "/Game/Blueprints/Multiplayer/BP_MP_PlayerController Object Reference"))
  (if (`KismetArrayLibrary.Array_Contains` (`self.Players`) Controller)
    (`KismetArrayLibrary.Array_Add` (`self.SpawnWaitingPlayers`) Controller)))

(fn `SpawnPlayers`
  (params (PlayersToSpawn :type "Array of /Game/Blueprints/Multiplayer/BP_MP_PlayerController Object Reference"))
  (locals (TEMP_NewPawns :type "Array of /Game/Blueprints/Multiplayer/BP_MP_PlayerCharacter Object Reference"))
  (bind _outactors (`GameplayStatics.GetAllActorsOfClass` "/Script/Engine.PlayerStart"))
  (for (_array_element _array_index) PlayersToSpawn
    (bind _possessed_pawn (`/Game/Blueprints/Multiplayer/BP_MP_PlayerController.Possessed Pawn` _array_element))
    (`/Engine/EditorBlueprintResources/StandardMacros.IsValid` _possessed_pawn
      (:`Is Valid`
        (`self.K2_DestroyActor` _possessed_pawn))
      (:`Is Not Valid`
        _))
    (bind _returnvalue (`|SpawnActorFromClass` "/Game/Blueprints/Multiplayer/BP_MP_PlayerCharacter.BP_MP_PlayerCharacter_C" (`self.GetTransform` (`|GetArrayItem` _outactors _array_index)) "AdjustIfPossibleButAlwaysSpawn" "OverrideRootScale" null null))
    (`KismetArrayLibrary.Array_Add` (`self.PlayerPawns`) _returnvalue)
    (`Controller.Possess` _array_element _returnvalue)
    (`KismetArrayLibrary.Array_Add` (`local.TEMP_NewPawns`) _returnvalue)
    (`/Game/Blueprints/Multiplayer/BP_MP_PlayerController.CLIENT Change Mode` _array_element "NewEnumerator1"))
  (`self.NotifyPawnSpawn` (`local.TEMP_NewPawns`)))

(fn `UserConstructionScript`)