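; Multiplayer player controller that owns the local HUD and relays player actions between client and server.
; On BeginPlay the local controller creates a collapsed HUD, which client mode changes show for playing and hide for spectating.
; Crosshair updates go straight to the HUD, and subtitles route through a client event.
; Interact, teleport and sound-on-actor requests forward to server events, the latter two acting on any supplied actor.
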(event `self.ReceiveBeginPlay`
  ;[1 0.7581 0.1451 1 30] Begin Play
  (`|ExecutionSequence`
    (:`then_0`
      (if (`self.IsLocalController`)
        (`self.CreateHUD`)))))

(event `/Game/Blueprints/Interfaces/IF_Actions.UpdateCrosshair`
  (params (bHovering :type Boolean) (Name :type "/Game/Data/STRUCT_LocalizedText Structure") (ELanguage :type "/Game/Data/ENUM_Language Enum" :default "NewEnumerator0") (EAction :type "/Game/Data/ENUM_ActionType Enum" :default "NewEnumerator0"))
  (`/Game/UI/Components/WBP_Crosshair.UpdateCrosshair` (`/Game/UI/WBP_HUD.WBP_Crosshair` (`self.W_HUD`)) bHovering Name ELanguage EAction))

(event `/Game/Blueprints/Interfaces/IF_Actions.ShowSubtitleAction`
  (params (Subtitle :type "/Game/Data/STRUCT_LocalizedText Structure") (IsPersistent :type Boolean) (HighlightText :type "/Game/Data/STRUCT_LocalizedText Structure") (HighlightColor :type "LinearColor Structure"))
  (`self.CLIENT_ShowSubtitle` Subtitle IsPersistent HighlightText HighlightColor))

(event `/Game/Blueprints/Interfaces/IF_Interaction.Interact`
  (params (Actor :type "Actor Object Reference") (PlayerController :type "PlayerController Object Reference") (IsLocked :type Boolean) (DidOpenInventory :type Boolean))
  (`self.SERVER Interact` Actor IsLocked DidOpenInventory))

(event `self.ReceivePossess`
  (params (PossessedPawn :type "Pawn Object Reference"))
  (set `self.Possessed Pawn` PossessedPawn))

(event `/Game/Blueprints/Interfaces/IF_Actions.Teleport`
  (params (Actor :type "Actor Object Reference") (Location :type "Vector Structure"))
  (`self.SERVER Teleport` Actor Location))

(event `/Game/Blueprints/Interfaces/IF_Actions.PlaySoundOnActor`
  (params (Actor :type "Actor Object Reference") (Sound :type "SoundCue Object Reference") (Location :type "Vector Structure"))
  (`self.SERVER Play Sound on Actor` Actor Sound Location))

(event `CLIENT Event Pawns Spawn`
  (params (Pawns :type "Array of /Game/Blueprints/Multiplayer/BP_MP_PlayerCharacter Object Reference"))
  (for _array_element Pawns
    (`/Game/Blueprints/Multiplayer/BP_MP_PlayerCharacter.Event Spawned` _array_element)))

(event `CLIENT Change Mode`
  (params (NewMode :type "/Game/Data/Multiplayer/ENUM_MP_PlayerMode Enum" :default "NewEnumerator0"))
  (bind _w_hud (`self.W_HUD`))
  (bind _output_get (set `self.CurrentMode` NewMode))
  (switch `/Game/Data/Multiplayer/ENUM_MP_PlayerMode` _output_get
    (:`NewEnumerator0`
      (`Widget.SetVisibility` _w_hud "Collapsed"))
    (:`NewEnumerator1`
      (`Widget.SetVisibility` _w_hud "HitTestInvisible"))))

(event `SERVER Interact`
  (params (Actor :type "Actor Object Reference") (IsLocked :type Boolean) (DidOpenInventory :type Boolean))
  (message `/Game/Blueprints/Interfaces/IF_Interaction.Interact` Actor null self IsLocked DidOpenInventory))

(event `CLIENT_ShowSubtitle`
  (params (Text :type "/Game/Data/STRUCT_LocalizedText Structure") (NewIsPersistent :type Boolean) (HighlightText :type "/Game/Data/STRUCT_LocalizedText Structure") (HighlightColor :type "LinearColor Structure"))
  (`/Game/UI/Components/WBP_Subtitles.ShowSubtitle` (`/Game/UI/WBP_HUD.WBP_Subtitles` (`self.W_HUD`)) Text (`/Game/Blueprints/Lib/GameLibrary.GetLanguage`) NewIsPersistent HighlightText HighlightColor))

(event `SERVER Teleport`
  (params (Actor :type "Actor Object Reference") (Location :type "Vector Structure"))
  (`self.K2_SetActorLocation` Actor Location false true))

(event `SERVER Play Sound on Actor`
  (params (Actor :type "Actor Object Reference") (Sound :type "SoundCue Object Reference") (Location :type "Vector Structure"))
  (message `/Game/Blueprints/Interfaces/IF_Actions.PlaySoundOnActor` Actor null Sound Location))

(fn `CreateHUD`
  (bind _returnvalue (`|CreateWidget` "/Game/UI/WBP_HUD.WBP_HUD_C" self))
  (bind _output_get (set `self.W_HUD` _returnvalue))
  (`UserWidget.AddToViewport` _output_get 0)
  (`Widget.SetVisibility` (`self.W_HUD`) "Collapsed"))

(fn `GetActorEnvironmentBody`
  (returns (Environment :type "/Game/Data/ENUM_EnvironmentBody Enum"))
  (return "NewEnumerator0"))

(fn `GetIsHidden`
  (returns (IsHidden :type Boolean))
  (return false))

(fn `GetSpeed`
  (returns (Speed :type "Float (double-precision)"))
  (return 0.0))

(fn `UserConstructionScript`)