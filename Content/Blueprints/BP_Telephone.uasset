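; BP_Telephone is an interactable save point that can also spawn the player back at its location.
; Opening interaction enables input, so pressing Interaction saves the current level name and player inventory to the GameInstance's current slot.
; SaveGame binds a completion callback after issuing the save, which prints a confirmation.
; SpawnPlayer forwards a saved inventory to a child-actor BP_PlayerTeleporter cached on BeginPlay.
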(event `self.ReceiveBeginPlay`
  (bind _asbp_game_instance (cast `/Game/Blueprints/BP_GameInstance` (`GameplayStatics.GetGameInstance`)))
  (set `self.GameInstance` _asbp_game_instance)
  (bind _asbp_player_teleporter (cast `/Game/Blueprints/BP_PlayerTeleporter` (`ChildActorComponent.ChildActor` (`self.Spawner`))))
  (set `self.PlayerSpawner` _asbp_player_teleporter))

(event `/Game/Blueprints/Interfaces/IF_Interaction.OpenInteraction`
  (`self.EnableInput` (`GameplayStatics.GetPlayerController` 0)))

(event `/Game/Blueprints/Interfaces/IF_Interaction.CloseInteraction`
  (`self.DisableInput` (`GameplayStatics.GetPlayerController` 0)))

(event `InputAction|Interaction`
  (params (Key :type "Key Structure"))
  (:`Pressed`
    (`self.SaveGame` (delegate `OnSaved`))))

(event `OnSaved`
  (`KismetSystemLibrary.PrintString` "TELEPHONE SAVED!" true true (struct :`G` 0.07963 :`B` 1.0 :`A` 1.0)))

(fn `GetSaveData`
  (returns (Data :type "/Game/Data/STRUCT_SaveData Structure"))
  (return (make `/Game/Data/STRUCT_SaveData` (`self.CurrentLevelName`) (`/Game/Blueprints/Components/InventoryComponent.Items` (`self.GetComponentByClass` (`GameplayStatics.GetPlayerPawn` 0) "/Game/Blueprints/Components/InventoryComponent.InventoryComponent_C")))))

(fn `SaveGame`
  (params (OnGameSaved :type "Delegate (by ref)"))
  (bind _gameinstance (`self.GameInstance`))
  (`/Game/Blueprints/BP_GameInstance.SaveGame` _gameinstance (`/Game/Blueprints/BP_GameInstance.GetCurrentSaveSlot` (`self.GameInstance`)) (`self.GetSaveData`))
  (add `/Game/Blueprints/BP_GameInstance.OnGameSaved` _gameinstance OnGameSaved))

(fn `SpawnPlayer`
  (params (SavedInventory :type "Array of /Game/Data/STRUCT_InventoryItem Structure (by ref)"))
  (`/Game/Blueprints/BP_PlayerTeleporter.SpawnPlayer` (`self.PlayerSpawner`) SavedInventory))

(fn `UserConstructionScript`
  (`/Game/Blueprints/Components/InteractionComponent.Setup` (`self.InteractionComponent`) (make `/Game/Data/STRUCT_LocalizedText` "telephone" "telefone") "NewEnumerator1"))