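; BP_Box is a destructible crate actor that can bring down other crates linked to it.
; Its Damage event subtracts from Health, playing a hit sound while health remains and calling DestroyBox once it reaches zero or below.
; DestroyBox recursively calls itself on each valid entry in DependantBoxes, then plays a break sound and destroys the actor.
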(event `/Game/Blueprints/Interfaces/IF_Damage.Damage`
  (params (Damage :type Integer))
  (bind _output_get (set `self.Health` (- (`self.Health`) Damage)))
  (if (<= _output_get 0)
    (`self.DestroyBox`)
    (else
      (`GameplayStatics.PlaySoundAtLocation` "/Game/SFX/Files/Interaction/SC_CRATE_HIT.SC_CRATE_HIT" (`self.K2_GetActorLocation`) (struct) 1.0 1.0 0.0 null null null null))))

(event `DestroyBox`
  (for _array_element (`self.DependantBoxes`)
    (`/Engine/EditorBlueprintResources/StandardMacros.IsValid` _array_element
      (:`Is Valid`
        (`self.DestroyBox` _array_element))))
  (`GameplayStatics.PlaySoundAtLocation` "/Game/SFX/Files/Interaction/SC_CRATE_BREAK.SC_CRATE_BREAK" (`self.K2_GetActorLocation`) (struct) 1.0 1.0 0.0 null null null null)
  (`self.K2_DestroyActor`))

(fn `UserConstructionScript`)