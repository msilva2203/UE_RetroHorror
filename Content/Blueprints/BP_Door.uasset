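; Interactable door that shows a HUD prompt on overlap and moves the player to an exit door or another level.
; Interaction runs once until reset and checks CanOpen, playing a lock sound and subtitle on failure.
; On success, it disables input and fall damage, then a transition widget's callback either teleports through the exit door's child-actor teleporter or hands off to BP_GameMode.
; The construction script copies a referenced actor's mesh and transform.
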(event `self.ReceiveBeginPlay`
  (bind _asbp_player_controller (cast `/Game/Blueprints/BP_PlayerController` (`GameplayStatics.GetPlayerController` 0)))
  (set `self.PlayerController` _asbp_player_controller))

(event `self.Collision.OnComponentBeginOverlap`
  (params (OverlappedComponent :type "PrimitiveComponent Object Reference") (OtherActor :type "Actor Object Reference") (OtherComp :type "PrimitiveComponent Object Reference") (OtherBodyIndex :type Integer) (bFromSweep :type Boolean) (SweepResult :type "HitResult Structure (by ref)"))
  (bind _asbp_player_character (cast `/Game/Blueprints/BP_PlayerCharacter` OtherActor))
  (set `self.PlayerCharacter` _asbp_player_character)
  (`self.EnableInput` (`GameplayStatics.GetPlayerController` 0))
  (bind _playercontroller (`self.PlayerController`)
    (:`then`
      (`/Game/Blueprints/BP_PlayerController.UpdateHUDPrompt` _playercontroller true (`self.Hints`)))
    (:`else`)))

(event `self.Collision.OnComponentEndOverlap`
  (params (OverlappedComponent :type "PrimitiveComponent Object Reference") (OtherActor :type "Actor Object Reference") (OtherComp :type "PrimitiveComponent Object Reference") (OtherBodyIndex :type Integer))
  (bind _asbp_player_character (cast `/Game/Blueprints/BP_PlayerCharacter` OtherActor))
  (set `self.PlayerCharacter` _asbp_player_character)
  (`self.DisableInput` (`GameplayStatics.GetPlayerController` 0))
  (bind _playercontroller (`self.PlayerController`)
    (:`then`
      (`/Game/Blueprints/BP_PlayerController.UpdateHUDPrompt` _playercontroller false (`self.Hints`)))
    (:`else`)))

(event `InputAction|Interaction`
  (params (Key :type "Key Structure"))
  (:`Pressed`
    (`/Engine/EditorBlueprintResources/StandardMacros.DoOnce` false :!label _label
      (:`Completed`
        (if (`self.CanOpen`)
          (`self.StartTransition` (delegate `OnTransition`))
          (else
            (`GameplayStatics.PlaySound2D` "/Game/SFX/SC_LOCK.SC_LOCK" 1.0 1.0 0.0 null null)
            (`self.ResetDoor`)
            (`/Game/Blueprints/BP_PlayerController.ShowSubtitle` (`self.PlayerController`) (`self.LockedMessage`))))))))

(event `ResetDoor`
  (goto _label :!via `Reset`))

(event `OnTransition`
  (if (`self.UseLevelTransition`)
    (`self.Transition`)
    (else
      (bind _asbp_player_teleporter (cast `/Game/Blueprints/BP_PlayerTeleporter` (`ChildActorComponent.ChildActor` (`/Game/Blueprints/BP_Door.Teleporter` (`self.ExitDoorReference`)))))
      (`self.EndTransition` (`self.PlayerCharacter`) (`self.Widget_Transition`) _asbp_player_teleporter))))

(fn `EndTransition`
  (params (CurrentPlayer :type "/Game/Blueprints/BP_PlayerCharacter Object Reference") (CurrentWidget :type "/Game/UI/Components/WBP_Transition Object Reference") (Teleporter :type "/Game/Blueprints/BP_PlayerTeleporter Object Reference"))
  (bind _currentplayer (`local.CurrentPlayer`))
  (`/Game/Blueprints/BP_PlayerTeleporter.TeleportPlayer` Teleporter (`local.CurrentPlayer`))
  (`GameplayStatics.PlaySound2D` "/Game/SFX/SC_DOOR.SC_DOOR" 1.0 1.0 0.0 null null)
  (`self.EnableInput` _currentplayer (`GameplayStatics.GetPlayerController` 0))
  (`/Game/Blueprints/Components/BasicCharacterComponent.SetFallDamageEnabled` (`/Game/Blueprints/BP_PlayerCharacter.Basic Character Component` _currentplayer) true)
  (`self.ResetDoor`)
  (`/Game/UI/Components/WBP_Transition.PlayAnim` (`local.CurrentWidget`) "Reverse"))

(fn `GetPlayerHasKey`
  (returns (HasKey :type Boolean))
  (bind _playercharacter (`self.PlayerCharacter`)
    (:`then`
      (return (`/Game/Blueprints/Components/InventoryComponent.HasKey` (`/Game/Blueprints/BP_PlayerCharacter.InventoryComponent` _playercharacter) (`KismetMathLibrary.Conv_ByteToInt` (`self.KeyItem`)))))
    (:`else`
      (return false))))

(fn `GetSelfTeleporter`
  (returns (Teleporter :type "/Game/Blueprints/BP_PlayerTeleporter Object Reference"))
  (return (cast `/Game/Blueprints/BP_PlayerTeleporter` (`ChildActorComponent.ChildActor` (`self.Teleporter`)) :!pure true)))

(fn `GetTag`
  (returns (TransitionTag :type Text))
  (return (`self.TransitionTag`)))

(fn `PlayTransition`
  (params (OnTransition :type "Delegate (by ref)"))
  (bind _widget_transition (`self.Widget_Transition`))
  (bind _returnvalue (`|CreateWidget` "/Game/UI/Components/WBP_Transition.WBP_Transition_C" (`GameplayStatics.GetPlayerController` 0)))
  (set `self.Widget_Transition` _returnvalue)
  (`UserWidget.AddToViewport` _widget_transition 999)
  (`/Game/UI/Components/WBP_Transition.PlayAnim` _widget_transition "Forward")
  (add `/Game/UI/Components/WBP_Transition.Transition` _widget_transition OnTransition))

(fn `StartTransition`
  (params (Delegate :type Delegate))
  (bind _playercharacter (`self.PlayerCharacter`))
  (`self.DisableInput` _playercharacter (`GameplayStatics.GetPlayerController` 0))
  (`/Game/Blueprints/Components/BasicCharacterComponent.SetFallDamageEnabled` (`/Game/Blueprints/BP_PlayerCharacter.Basic Character Component` _playercharacter) false)
  (`self.PlayTransition` Delegate))

(fn `Transition`
  (bind _asbp_game_mode (cast `/Game/Blueprints/BP_GameMode` (`GameplayStatics.GetGameMode`)))
  (`/Game/Blueprints/BP_GameMode.TransitionLevels` _asbp_game_mode (`self.CurrentWorld`) (`self.NextWorld`) (make `/Game/Data/STRUCT_TransitionData` (`self.PlayerCharacter`) (`self.Widget_Transition`) (`self.TransitionTag`))))

(fn `UserConstructionScript`
  (bind _doormesh (`self.DoorMesh`))
  (bind _mesh (`self.Mesh`)
    (:`then`
      (`StaticMeshComponent.SetStaticMesh` _doormesh (`StaticMeshComponent.StaticMesh` (`StaticMeshActor.StaticMeshComponent` _mesh)))
      (`PrimitiveComponent.SetMaterial` _doormesh 0 "/Game/Materials/M_Interactable.M_Interactable")
      (`SceneComponent.K2_SetWorldTransform` _doormesh (`self.GetTransform` _mesh) false false))
    (:`else`)))