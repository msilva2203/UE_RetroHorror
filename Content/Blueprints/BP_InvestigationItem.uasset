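; BP_InvestigationItem is an interactable item that shows its message as a subtitle when the player investigates it.
; On begin play it sets up its InteractionComponent with the item's name and a fixed action type, and caches the BP_PlayerController.
; Open and close interaction events toggle the actor's input, so the Interaction key shows the non-persistent subtitle only while interaction is open.
; The construction script applies the configured item mesh.
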(event `self.ReceiveBeginPlay`
  (`/Game/Blueprints/Components/InteractionComponent.Setup` (`self.InteractionComponent`) (`self.Name`) "NewEnumerator3")
  (bind _asbp_player_controller (cast `/Game/Blueprints/BP_PlayerController` (`GameplayStatics.GetPlayerController` 0)))
  (set `self.PlayerController` _asbp_player_controller))

(event `/Game/Blueprints/Interfaces/IF_Interaction.OpenInteraction`
  (`self.EnableInput` (`self.PlayerController`)))

(event `/Game/Blueprints/Interfaces/IF_Interaction.CloseInteraction`
  (`self.DisableInput` (`self.PlayerController`)))

(event `InputAction|Interaction`
  (params (Key :type "Key Structure"))
  (:`Pressed`
    (`/Game/Blueprints/BP_PlayerController.ShowSubtitle` (`self.PlayerController`) (`self.Message`) false)))

(fn `UserConstructionScript`
  (`StaticMeshComponent.SetStaticMesh` (`self.Mesh`) (`self.ItemMesh`)))