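; GameLibrary is a Blueprint function library that gives global access to game instance settings.
; GetGameInstance casts the current game instance to BP_GameInstance.
; GetInputDevice and GetLanguage use that helper to return the instance's current input device and language.
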(fn `GetGameInstance`
  (returns (GameInstance :type "/Game/Blueprints/BP_GameInstance Object Reference"))
  (return (cast `/Game/Blueprints/BP_GameInstance` (`GameplayStatics.GetGameInstance` (`local.__WorldContext`)) :!pure true)))

(fn `GetInputDevice`
  (returns (inputDevice :type "/Game/Data/ENUM_InputDevice Enum"))
  (return (`/Game/Blueprints/BP_GameInstance.GetInputDevice` (`self.GetGameInstance` (`local.__WorldContext`)))))

(fn `GetLanguage`
  (returns (Language :type "/Game/Data/ENUM_Language Enum"))
  (return (`/Game/Blueprints/BP_GameInstance.GetLanguage` (`self.GetGameInstance` (`local.__WorldContext`)))))