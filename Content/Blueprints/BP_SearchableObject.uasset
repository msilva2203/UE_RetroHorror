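; BP_SearchableObject is a world object the player searches once by holding the Interaction input to receive an item.
; Opening interaction enables input on the actor, while closing disables it and reverses the hold.
; A timeline plays while held and reverses on release, printing progress; finishing forward adds one fixed item to the pawn's InventoryComponent and sets Searched.
; The construction script applies the chosen mesh to a base and a BrightMesh using M_Interactable.
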(event `/Game/Blueprints/Interfaces/IF_Interaction.OpenInteraction`
  (`self.EnableInput` (`GameplayStatics.GetPlayerController` 0)))

(event `/Game/Blueprints/Interfaces/IF_Interaction.CloseInteraction`
  (`self.DisableInput` (`GameplayStatics.GetPlayerController` 0))
  (`self.StopHold`))

(event `InputAction|Interaction`
  (params (Key :type "Key Structure"))
  (:`Pressed`
    (`self.StartHold`))
  (:`Released`
    (`self.StopHold`)))

(event `StartHold`
  (if (not (`self.Searched`))
    (bind (_direction _holdprogress) (`Timeline|Timeline_Hold` :!label _label)
      (:`Update`
        (`KismetSystemLibrary.PrintString` (`KismetStringLibrary.Conv_DoubleToString` _holdprogress)))
      (:`Finished`
        (switch `ETimelineDirection` _direction
          (:`Forward`
            (`/Game/Blueprints/Components/InventoryComponent.AddToInventory` (`self.GetComponentByClass` (`Controller.K2_GetPawn` (`GameplayStatics.GetPlayerController` 0)) "/Game/Blueprints/Components/InventoryComponent.InventoryComponent_C") "NewEnumerator1" 1)
            (set `self.Searched` true)))))))

(event `StopHold`
  (goto _label :!via `Reverse`))

(fn `UserConstructionScript`
  (`StaticMeshComponent.SetStaticMesh` (`self.Static Mesh`) (`self.Mesh`))
  (`StaticMeshComponent.SetStaticMesh` (`self.BrightMesh`) (`self.Mesh`))
  (`PrimitiveComponent.SetMaterial` (`self.BrightMesh`) 0 "/Game/Materials/M_Interactable.M_Interactable"))