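; BP_ItemSearchable is a world object that the player searches by holding Interaction to receive an item once.
; Its InteractionComponent is set up on BeginPlay, and opening or closing the interaction toggles the actor's input.
; Holding plays a timeline that drives the HUD search box, and releasing reverses it.
; Completing the timeline adds the Item and Quantity to the pawn's inventory, marks it searched and disables the mesh's custom depth.
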(event `self.ReceiveBeginPlay`
  (`/Game/Blueprints/Components/InteractionComponent.Setup` (`self.InteractionComponent`) (`self.Name`) "NewEnumerator1")
  (bind _asbp_player_controller (cast `/Game/Blueprints/BP_PlayerController` (`GameplayStatics.GetPlayerController` 0)))
  (set `self.PlayerController` _asbp_player_controller))

(event `/Game/Blueprints/Interfaces/IF_Interaction.OpenInteraction`
  (`self.EnableInput` (`GameplayStatics.GetPlayerController` 0))
  (set `self.IsInputEnabled` true))

(event `/Game/Blueprints/Interfaces/IF_Interaction.CloseInteraction`
  (`self.DisableInput` (`GameplayStatics.GetPlayerController` 0))
  (set `self.IsInputEnabled` false)
  (`self.StopHold`)
  (`/Game/UI/Components/WBP_SearchBox.SetIsVisible` (`self.GetSearchWidget`) false)
  (`self.ResetBar`))

(event `InputAction|Interaction`
  (params (Key :type "Key Structure"))
  (:`Pressed`
    (`self.StartHold`)
    (`/Engine/EditorBlueprintResources/StandardMacros.DoOnce` false :!label _label
      (:`Completed`
        (if (not (`self.Searched`))
          (`/Game/UI/Components/WBP_SearchBox.SetIsVisible` (`self.GetSearchWidget`) true)))))
  (:`Released`
    (`self.StopHold`)))

(event `ResetBar`
  (goto _label :!via `Reset`))

(event `StartHold`
  (if (not (`self.Searched`))
    (bind (_direction _holdprogress) (`Timeline|Timeline_Hold` :!label _label_2)
      (:`Update`
        (`/Game/UI/Components/WBP_SearchBox.UpdateProgress` (`/Game/UI/WBP_HUD.WBP_SearchBox` (`/Game/Blueprints/BP_PlayerController.GetPlayerHUD` (`self.PlayerController`))) _holdprogress))
      (:`Finished`
        (switch `ETimelineDirection` _direction
          (:`Forward`
            (`/Game/Blueprints/Components/InventoryComponent.AddToInventory` (`self.GetComponentByClass` (`Controller.K2_GetPawn` (`GameplayStatics.GetPlayerController` 0)) "/Game/Blueprints/Components/InventoryComponent.InventoryComponent_C") (`self.Item`) (`self.Quantity`))
            (set `self.Searched` true)
            (`PrimitiveComponent.SetRenderCustomDepth` (`self.Static Mesh`) false)))))))

(event `StopHold`
  (if (not (`self.Searched`))
    (goto _label_2 :!via `Reverse`)))

(fn `GetSearchWidget`
  (returns (WBP_SearchBox :type "/Game/UI/Components/WBP_SearchBox Object Reference"))
  (return (`/Game/UI/WBP_HUD.WBP_SearchBox` (`/Game/Blueprints/BP_PlayerController.GetPlayerHUD` (`self.PlayerController`)))))

(fn `UserConstructionScript`
  (`StaticMeshComponent.SetStaticMesh` (`self.Static Mesh`) (`self.Mesh`)))