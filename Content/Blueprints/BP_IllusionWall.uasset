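; BP_IllusionWall is a fake wall that vanishes when pushed or damaged.
; Both triggers call DiscoverWall, which runs once, plays a timeline fading the dynamic material's Opacity, then destroys the actor.
; Collision on the front and back meshes switches off shortly after the fade starts.
; The construction script gives both meshes one shared dynamic material instance; GetIsHidden and GetSpeed return fixed defaults.
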(event `/Game/Blueprints/Interfaces/IF_Actions.Push`
  (`self.DiscoverWall` :!label _label))

(event `/Game/Blueprints/Interfaces/IF_Damage.Damage`
  (params (Damage :type Integer))
  (goto _label))

(event `DiscoverWall`
  (`/Engine/EditorBlueprintResources/StandardMacros.DoOnce` false
    (:`Completed`
      (`|ExecutionSequence`
        (:`then_0`
          (bind (_direction _opacity) (`Timeline|Timeline_WallFade`)
            (:`Update`
              (`MaterialInstanceDynamic.SetScalarParameterValue` (`self.InstancedMaterial`) "Opacity" _opacity))
            (:`Finished`
              (`self.K2_DestroyActor`))))
        (:`then_1`
          (`KismetSystemLibrary.Delay` 0.35)
          (`PrimitiveComponent.SetCollisionEnabled` (`self.WallBack`) "NoCollision")
          (`PrimitiveComponent.SetCollisionEnabled` (`self.WallFront`) "NoCollision"))))))

(fn `GetIsHidden`
  (returns (IsHidden :type Boolean))
  (return false))

(fn `GetSpeed`
  (returns (Speed :type "Float (double-precision)"))
  (return 0.0))

(fn `UserConstructionScript`
  (bind _returnvalue (`KismetMaterialLibrary.CreateDynamicMaterialInstance` (`self.WallMaterial`)))
  (bind _output_get (set `self.InstancedMaterial` _returnvalue))
  (`PrimitiveComponent.SetMaterial` (`self.WallBack`) 0 _output_get)
  (`PrimitiveComponent.SetMaterial` (`self.WallFront`) 0 _output_get))