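; BP_Car is a drivable car pawn that the first player possesses through OpenInteraction, while CloseInteraction only disables input.
; Forward and right axis input accumulate into clamped speed and turn values with no decay.
; Each tick pushes the Car component along the negative right vector with both acceleration force and velocity-change impulse.
; Steering adds world yaw every tick, unscaled by delta time.
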(event `self.ReceiveTick`
  (params (DeltaSeconds :type "Float (single-precision)"))
  (bind _output_get (set `self.Speed` (`KismetMathLibrary.FClamp` (+ (* (`self.GetInputAxisValue`) DeltaSeconds (`self.SpeedIncerment`)) (`self.Speed`)) -50.0 200.0)))
  (bind _returnvalue (* (`self.GetActorRightVector`) _output_get -1.0))
  (`PrimitiveComponent.AddForce` (`self.Car`) _returnvalue "None" true)
  (`PrimitiveComponent.AddImpulse` (`self.Car`) _returnvalue "None" true)
  (`self.K2_AddActorWorldRotation` (`KismetMathLibrary.MakeRotator` 0.0 0.0 (`self.RightSpeed`))))

(event `InputAxis|MoveRight`
  (params (AxisValue :type "Float (single-precision)"))
  (set `self.RightSpeed` (`KismetMathLibrary.FClamp` (+ (* AxisValue (`GameplayStatics.GetWorldDeltaSeconds`) (`self.RightSpeedIncrement`)) (`self.RightSpeed`)) -50.0 50.0)))

(event `/Game/Blueprints/Interfaces/IF_Interaction.CloseInteraction`
  (params (PlayerController :type "PlayerController Object Reference"))
  (`self.DisableInput` PlayerController))

(event `/Game/Blueprints/Interfaces/IF_Interaction.OpenInteraction`
  (params (PlayerController :type "PlayerController Object Reference"))
  (bind _returnvalue (`GameplayStatics.GetPlayerController` 0))
  (`KismetSystemLibrary.PrintString` "Hello")
  (`Controller.UnPossess` _returnvalue)
  (`Controller.Possess` _returnvalue self)
  (`PlayerController.SetViewTargetWithBlend` _returnvalue self 0.0 "VTBlend_Linear" 0.0 false))

(event `InputAction|Interaction`
  (params (Key :type "Key Structure")))

(fn `GetCustomKeys`
  (returns (Keys :type "Array of Text"))
  (return))

(fn `UserConstructionScript`)