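; BP_LevelLight is a level lighting actor that applies day/night and weather changes, branching on an indoor flag.
; UpdateDay lerps six directional lights and retro post-process fog outdoors, or passes the day alpha to the level's window lights indoors.
; UpdateWeather fades rain audio, using a separate indoor loop, and outdoors toggles a rain effect with random spawn rate.
; Tick keeps that effect on the player.
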(event `self.ReceiveBeginPlay`
  (bind _outactors (`GameplayStatics.GetAllActorsOfClass` "/Game/Blueprints/Misc/BP_WindowLight.BP_WindowLight_C"))
  (set `self.WindowLights` _outactors)
  (if (not (`self.IsIndoor`))
    (bind _returnvalue (`NiagaraFunctionLibrary.SpawnSystemAtLocation` "/Game/Particles/VFX_Rain.VFX_Rain" (0.0 0.0 0.0) (struct) (1.0 1.0 1.0) false false))
    (set `self.System_Rain` _returnvalue)
    (`self.SetActorTickEnabled` true)))

(event `self.ReceiveTick`
  (params (DeltaSeconds :type "Float (single-precision)"))
  (bind _returnvalue (`GameplayStatics.GetPlayerCharacter` 0))
  (`/Engine/EditorBlueprintResources/StandardMacros.IsValid` _returnvalue
    (:`Is Valid`
      (`SceneComponent.K2_SetWorldLocation` (`self.System_Rain`) (`self.K2_GetActorLocation` _returnvalue) false false))))

(event `self.ReceiveEndPlay`
  (params (EndPlayReason :type "EEndPlayReason Enum" :default "Destroyed"))
  (bind _system_rain (`self.System_Rain`)
    (:`then`
      (`ActorComponent.K2_DestroyComponent` _system_rain))
    (:`else`)))

(fn `GetIsIndoor`
  (returns (IsIndoor :type Boolean))
  (return (`self.IsIndoor`)))

(fn `GetWeatherSound`
  (params (NewWeather :type "/Game/Data/ENUM_Weather Enum" :default "NewEnumerator0"))
  (returns (Sound :type "SoundCue Object Reference"))
  (return (select `/Game/Data/ENUM_Weather` (`local.NewWeather`) :`NewEnumerator1` (select `bool` (`self.IsIndoor`) :`false` "/Game/SFX/SC_RAIN_LOOP.SC_RAIN_LOOP" :`true` "/Game/SFX/SC_RAIN_INDOOR_LOOP.SC_RAIN_INDOOR_LOOP" :!type "SoundCue Object Reference"))))

(fn `SetLightIntensity`
  (params (NewIntensity :type "Float (single-precision)"))
  (`LightComponent.SetIntensity` (`self.DirectionalLight1`) NewIntensity)
  (`LightComponent.SetIntensity` (`self.DirectionalLight2`) NewIntensity)
  (`LightComponent.SetIntensity` (`self.DirectionalLight3`) NewIntensity)
  (`LightComponent.SetIntensity` (`self.DirectionalLight4`) NewIntensity)
  (`LightComponent.SetIntensity` (`self.DirectionalLight5`) NewIntensity)
  (`LightComponent.SetIntensity` (`self.DirectionalLight`) NewIntensity))

(fn `UpdateDay`
  (params (DayAlpha :type "Float (double-precision)"))
  (bind _dayalpha (`local.DayAlpha`))
  (if (`self.IsIndoor`)
    (`self.UpdateWindowLights` (`local.DayAlpha`))
    (else
      (`self.SetLightIntensity` (`KismetMathLibrary.Lerp` (`self.MinIntensity`) (`self.MaxIntensity`) (`local.DayAlpha`)))
      (`self.UpdateFog` (`KismetMathLibrary.LinearColorLerp` (`self.Fog Color Night`) (`self.Fog Color Day`) _dayalpha) (`KismetMathLibrary.Lerp` (`self.Start Offset Night`) (`self.Start Offset`) _dayalpha)))))

(fn `UpdateFog`
  (params (FogColor :type "LinearColor Structure") (StartOffset :type "Float (double-precision)"))
  (bind _retrobp (`self.RetroBP`))
  (`/Engine/EditorBlueprintResources/StandardMacros.IsValid` _retrobp
    (:`Is Valid`
      (`/Game/Materials/RetroShadersV4/RetroShader/BP_RetroPostProcess.SetFogParameters` _retrobp true FogColor StartOffset (`self.Fog Distance`) (`self.Noise Strength`) (`self.Noise Scale`) (`self.Noise Direction`)))))

(fn `UpdateWeather`
  (params (NewWeather :type "/Game/Data/ENUM_Weather Enum" :default "NewEnumerator0"))
  (bind _weatheraudio (`self.WeatherAudio`))
  (bind _system_rain (`self.System_Rain`))
  (`KismetSystemLibrary.PrintString` (`|GetEnumeratorNameAsString` NewWeather))
  (if (`|EnumEquality` NewWeather "NewEnumerator0")
    (`AudioComponent.FadeOut` (`self.WeatherAudio`) 1.0 0.0 "Linear")
    (if (not (`self.IsIndoor`))
      (`ActorComponent.Deactivate` (`self.System_Rain`)))
    (else
      (`AudioComponent.SetSound` _weatheraudio (`self.GetWeatherSound` NewWeather))
      (`AudioComponent.FadeIn` _weatheraudio 1.0 1.0 0.0 "Linear")
      (if (not (`self.IsIndoor`))
        (`ActorComponent.Activate` _system_rain true)
        (`FXSystemComponent.SetFloatParameter` _system_rain "SpawnRate" (`KismetMathLibrary.RandomFloatInRange` 1000.0 2500.0))))))

(fn `UpdateWindowLights`
  (params (DayAlpha :type "Float (double-precision)"))
  (for _array_element (`self.WindowLights`)
    (`/Game/Blueprints/Misc/BP_WindowLight.UpdateIntesity` _array_element (`local.DayAlpha`))))

(fn `UserConstructionScript`
  (`self.SetLightIntensity` (`self.MaxIntensity`))
  (set `self.RetroBP` (cast `/Game/Materials/RetroShadersV4/RetroShader/BP_RetroPostProcess` (`ChildActorComponent.ChildActor` (`self.RetroPP`)) :!pure true))
  (`self.UpdateFog` (`self.Fog Color Day`) (`self.Start Offset`))
  (if (`self.IsIndoor`)
    (set `self.MinIntensity` (`self.MaxIntensity`))))