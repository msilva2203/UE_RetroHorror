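; BP_Bush is a foliage actor that tilts its mesh and plays a bush sound when the player character walks into it.
; CollisionBox overlaps store the player, toggle IsColliding and trigger the sound on entry.
; Tick lerps the mesh's world rotation toward a quarter-scaled look-at rotation derived from the player offset, or back to zero rotation once the overlap ends, at a rate set by Speed.
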(event `self.ReceiveTick`
  (params (DeltaSeconds :type "Float (single-precision)"))
  (`self.PlayerCharacter`
    (:`then`
      (`SceneComponent.K2_SetWorldRotation` (`self.BushMesh`) (`KismetMathLibrary.RLerp` (`SceneComponent.K2_GetComponentRotation` (`self.BushMesh`)) (`KismetMathLibrary.SelectRotator` (* (`KismetMathLibrary.FindLookAtRotation` (- (`self.K2_GetActorLocation`) (`self.K2_GetActorLocation` (`self.PlayerCharacter`))) (`KismetMathLibrary.Vector_Up`)) 0.25) (struct) (`self.IsColliding`)) (* DeltaSeconds (`self.Speed`))) false false))
    (:`else`)))

(event `self.CollisionBox.OnComponentBeginOverlap`
  (params (OverlappedComponent :type "PrimitiveComponent Object Reference") (OtherActor :type "Actor Object Reference") (OtherComp :type "PrimitiveComponent Object Reference") (OtherBodyIndex :type Integer) (bFromSweep :type Boolean) (SweepResult :type "HitResult Structure (by ref)"))
  (bind _asbp_player_character (cast `/Game/Blueprints/BP_PlayerCharacter` OtherActor))
  (set `self.PlayerCharacter` _asbp_player_character)
  (set `self.IsColliding` true)
  (`GameplayStatics.PlaySoundAtLocation` "/Game/SFX/SC_BUSH.SC_BUSH" (`self.K2_GetActorLocation`) (struct) 1.0 1.0 0.0 null null null null))

(event `self.CollisionBox.OnComponentEndOverlap`
  (params (OverlappedComponent :type "PrimitiveComponent Object Reference") (OtherActor :type "Actor Object Reference") (OtherComp :type "PrimitiveComponent Object Reference") (OtherBodyIndex :type Integer))
  (bind _asbp_player_character (cast `/Game/Blueprints/BP_PlayerCharacter` OtherActor))
  (set `self.PlayerCharacter` _asbp_player_character)
  (set `self.IsColliding` false))

(fn `UserConstructionScript`)