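; BP_Post_Light is a placeable post light actor with an On, Off or Broken state.
; The construction script stretches the actor vertically and sets the light's visibility from that state, with Broken starting visible.
; At BeginPlay, a Broken light starts a self-calling Blink event that toggles visibility at random short intervals to create a faulty flicker.
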(event `self.ReceiveBeginPlay`
  (if (`|EnumEquality` (`self.LightState`) "NewEnumerator2")
    (`self.Blink`)))

(event `Blink`
  (bind _light (`self.Light`))
  (`SceneComponent.SetVisibility` _light (not (`SceneComponent.bVisible` _light)) false)
  (`KismetSystemLibrary.Delay` (`KismetMathLibrary.RandomFloatInRange` 0.5 2.0))
  (`self.Blink`))

(fn `UserConstructionScript`
  (`self.SetActorRelativeScale3D` (1.0 1.0 1.5))
  (`SceneComponent.SetVisibility` (`self.Light`) (select `/Game/Data/ENUM_LightState` (`self.LightState`) :`NewEnumerator0` true :`NewEnumerator2` true) false))