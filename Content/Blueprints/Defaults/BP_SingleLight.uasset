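; BP_SingleLight is a placeable light with a buzz sound and three states: On, Off and Broken.
; A cull collision volume enables it while a controlled pawn is inside and turns it off on exit.
; SetLightVisibility toggles Light and PointLight together and fades the buzz with them.
; Broken lights flicker through a self-calling Blink event with random delays, which stops once out of range.
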(event `self.ReceiveBeginPlay`
  (if (`self.InsideRange`)
    (`self.Activate`)
    (else
      (`self.SetLightVisibility` false))))

(event `Activate`
  (`self.SetLightVisibility` (select `/Game/Data/ENUM_LightState` (`self.LightState`) :`NewEnumerator0` true :`NewEnumerator2` true))
  (if (`|EnumEquality` (`self.LightState`) "NewEnumerator2")
    (`self.Blink`)))

(event `Blink`
  (if (`self.InsideRange`)
    (`self.SetLightVisibility` (not (`SceneComponent.bVisible` (`self.Light`))))
    (`KismetSystemLibrary.Delay` (`KismetMathLibrary.RandomFloatInRange` 0.75 1.5))
    (`self.Blink`)
    (else
      (`self.SetLightVisibility` false))))

(event `self.CullCollision.OnComponentBeginOverlap`
  (params (OverlappedComponent :type "PrimitiveComponent Object Reference") (OtherActor :type "Actor Object Reference") (OtherComp :type "PrimitiveComponent Object Reference") (OtherBodyIndex :type Integer) (bFromSweep :type Boolean) (SweepResult :type "HitResult Structure (by ref)"))
  (bind _aspawn (cast `Pawn` OtherActor))
  (if (`Pawn.IsControlled` _aspawn)
    (set `self.InsideRange` true)
    (`self.Activate`)))

(event `self.CullCollision.OnComponentEndOverlap`
  (params (OverlappedComponent :type "PrimitiveComponent Object Reference") (OtherActor :type "Actor Object Reference") (OtherComp :type "PrimitiveComponent Object Reference") (OtherBodyIndex :type Integer))
  (bind _aspawn (cast `Pawn` OtherActor))
  (if (`Pawn.IsControlled` _aspawn)
    (set `self.InsideRange` false)
    (`self.SetLightVisibility` false)))

(fn `SetLightVisibility`
  (params (bNewVisibility :type Boolean))
  (bind _audiobuzz (`self.AudioBuzz`))
  (`SceneComponent.SetVisibility` (`self.Light`) bNewVisibility false)
  (`SceneComponent.SetVisibility` (`self.PointLight`) bNewVisibility false)
  (if (`local.bNewVisibility`)
    (`AudioComponent.FadeIn` _audiobuzz 0.1 1.0 0.0 "Linear")
    (else
      (`AudioComponent.FadeOut` _audiobuzz 0.1 0.0 "Linear"))))

(fn `UserConstructionScript`
  (bind _returnvalue (select `/Game/Data/ENUM_LightState` (`self.LightState`) :`NewEnumerator0` true :`NewEnumerator2` true))
  (`self.SetActorRelativeScale3D` (1.5 1.5 1.5))
  (`self.SetLightVisibility` _returnvalue)
  (if _returnvalue
    (`ActorComponent.SetAutoActivate` (`self.AudioBuzz`) true)))