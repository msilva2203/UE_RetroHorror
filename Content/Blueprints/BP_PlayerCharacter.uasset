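; Player character for a horror-style game, handling movement, dodging, interaction, inventory, flashlight spawning, jumpscares and death with level reload.
; BasicCharacterComponent updates drive health and stamina post-process feedback, adrenaline-based heartbeat and FOV, and walk speed from stamina and adrenaline.
; Looping timers run footsteps, stamina regeneration and adrenaline decay.
; Line traces find interactables each tick through DoOnce gates, pick surface footstep sounds and shorten dodges at obstacles.
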(event `HandleInteraction`
  (bind _actor (`self.FindInteractionActor`))
  ;[1 0.7581 0.1451 1 20] Handle Interactions
  (if (`KismetSystemLibrary.DoesImplementInterface` _actor "/Game/Blueprints/Interfaces/IF_Interaction.IF_Interaction_C")
    (`/Engine/EditorBlueprintResources/StandardMacros.DoOnce` false :!label _label
      (:`Completed`
        (`|ExecutionSequence`
          (:`then_0`
            (bind _output_get (set `self.CurrentInteractable` _actor))
            (`/Game/Blueprints/Components/InteractionComponent.Open` (`self.GetComponentByClass` _output_get "/Game/Blueprints/Components/InteractionComponent.InteractionComponent_C")))
          (:`then_1`
            (goto _label_2 :!via `Reset`)))))
    (else
      (`/Engine/EditorBlueprintResources/StandardMacros.DoOnce` false :!label _label_2
        (:`Completed`
          (`|ExecutionSequence`
            (:`then_0`
              (bind _currentinteractable (`self.CurrentInteractable`)
                (:`then`
                  (`/Game/Blueprints/Components/InteractionComponent.Close` (`self.GetComponentByClass` _currentinteractable "/Game/Blueprints/Components/InteractionComponent.InteractionComponent_C"))
                  (set `self.CurrentInteractable` null))
                (:`else`
                  (`/Game/Blueprints/BP_PlayerController.HideCrosshair` (`self.PlayerController`)))))
            (:`then_1`
              (goto _label :!via `Reset`))))))))

(event `InitFooststeps`
  ;[1 0.7581 0.1451] Footsteps
  (bind _returnvalue (`KismetSystemLibrary.K2_SetTimerDelegate` (delegate `StepSound`) 0.75 true))
  (set `self.Timer_Foosteps` _returnvalue))

(event `InputAxis|MoveForward`
  (params (AxisValue :type "Float (single-precision)"))
  ;[1 0.7581 0.1451 1 25] Player Movement and Camera Controls
  (`self.AddMovementInput` (`self.GetPlayerForwardDirection`) AxisValue))

(event `InputAxis|LookUp`
  (params (AxisValue :type "Float (single-precision)"))
  ;[1 0.7581 0.1451 1 25] Player Movement and Camera Controls
  (`self.AddControllerPitchInput` (`self.GetPlayerPitchMultiplier` AxisValue)))

(event `StepSound`
  ;[1 0.7581 0.1451] Footsteps
  (if (and (> (`self.GetVelocityLength`) 0.0) (not (`NavMovementComponent.IsFalling` (`self.CharacterMovement`))))
    (`self.PlaySoundAtLocation` (`self.GetMaterialSound`))))

(event `InputAxis|MoveRight`
  (params (AxisValue :type "Float (single-precision)"))
  ;[1 0.7581 0.1451 1 25] Player Movement and Camera Controls
  (`self.AddMovementInput` (`self.GetPlayerRightDirection`) AxisValue))

(event `InputAxis|Turn`
  (params (AxisValue :type "Float (single-precision)"))
  ;[1 0.7581 0.1451 1 25] Player Movement and Camera Controls
  (`self.AddControllerYawInput` (`self.GetPlayerYawMultiplier` AxisValue)))

(event `InputAction|Jump`
  (params (Key :type "Key Structure"))
  ;[1 0.7581 0.1451 1 25] Player Movement and Camera Controls
  (:`Pressed`
    (`self.Jump`)))

(event `InputAction|Crouch`
  (params (Key :type "Key Structure"))
  ;[1 0.7581 0.1451 1 25] Player Movement and Camera Controls
  (:`Pressed`
    (`self.Crouch`))
  (:`Released`
    (`self.UnCrouch`)))

(event `StopStaminaRegen`
  (params (Time :type "Float (double-precision)"))
  ;[1 0.7581 0.1451] Stamina Regen and Pauses
  (`KismetSystemLibrary.K2_ClearAndInvalidateTimerHandle` (`self.Timer_StaminaRegen`))
  (`KismetSystemLibrary.K2_ClearAndInvalidateTimerHandle` (`self.Timer_StaminaStop`))
  (bind _returnvalue (`KismetSystemLibrary.K2_SetTimerDelegate` (delegate `InitStaminaRegen`) Time))
  (set `self.Timer_StaminaStop` _returnvalue))

(event `Jumpscare`
  (params (Adrenaline :type Integer) (Location :type "Vector Structure"))
  (bind _returnvalue (`GameplayStatics.GetPlayerController` 0))
  (bind _returnvalue_2 (`GameplayStatics.GetPlayerController` 0))
  (`/Game/Blueprints/Components/BasicCharacterComponent.OffsetAdrenaline` (`self.Basic Character Component`) Adrenaline)
  (`self.DisableInput` _returnvalue)
  (set `self.JumpscareRotation` (`Controller.GetControlRotation` _returnvalue))
  (`GameplayStatics.PlaySound2D` "/Game/SFX/SC_JUMPSCARE.SC_JUMPSCARE" 1.0 1.0 0.0 null null)
  (bind (_direction _alpha) (`Timeline|Timeline_Jumpscare` :!via `PlayFromStart`)
    (:`Update`
      (`Controller.SetControlRotation` _returnvalue_2 (`KismetMathLibrary.RLerp` (`self.JumpscareRotation`) (`KismetMathLibrary.FindLookAtRotation` (`self.K2_GetActorLocation`) Location) _alpha true)))
    (:`Finished`
      (`/Game/Blueprints/BP_PlayerController.ShowSubtitle` (`self.PlayerController`) (`KismetArrayLibrary.Array_Random` (`self.JumpscareMessages`)) false)
      (`KismetSystemLibrary.Delay` 0.2)
      (`self.EnableInput` _returnvalue_2))))

(event `InitStaminaRegen`
  ;[1 0.7581 0.1451] Stamina Regen and Pauses
  (bind _returnvalue (`KismetSystemLibrary.K2_SetTimerDelegate` (delegate `GainStamina`) 0.05 true))
  (set `self.Timer_StaminaRegen` _returnvalue))

(event `self.ReceiveBeginPlay`
  ;[1 0.7581 0.1451] Begin Play
  (`|ExecutionSequence`
    (:`then_0`
      (`self.InitFooststeps`))
    (:`then_1`
      (`self.InitStaminaRegen`))
    (:`then_2`
      (bind _asbp_player_controller (cast `/Game/Blueprints/BP_PlayerController` (`GameplayStatics.GetPlayerController` 0)))
      (set `self.PlayerController` _asbp_player_controller))
    (:`then_3`
      (`self.StartAdrenalineTimer`))))

(event `GainStamina`
  ;[1 0.7581 0.1451] Stamina Regen and Pauses
  (if (!= (`/Game/Blueprints/Components/BasicCharacterComponent.GetStaminaPercent` (`self.Basic Character Component`)) 1.0)
    (`/Game/Blueprints/Components/BasicCharacterComponent.OffsetStamina` (`self.Basic Character Component`) 1)))

(event `Key|Gamepad_RightShoulder`
  (params (Key :type "Key Structure"))
  (:`Pressed`
    (`|SpawnActorFromClass` "/Game/Blueprints/Equipment/BP_Flashlight.BP_Flashlight_C" (`self.GetTransform`) "Undefined" "OverrideRootScale" null null :!label _label_3)))

(event `Key|One`
  (params (Key :type "Key Structure"))
  (:`Pressed`
    (goto _label_3)))

(event `self.ReceiveTick`
  (params (DeltaSeconds :type "Float (single-precision)"))
  ;[1 0.7581 0.1451] Event Tick
  (`|ExecutionSequence`
    (:`then_0`
      (`self.HandleInteraction`))))

(event `self.Basic Character Component.OnHealthUpdate`
  (params (CurrentHealth :type Integer) (HealthPercent :type "Float (double-precision)") (Positive :type Boolean))
  (`self.UpdateHealthFeedback` HealthPercent)
  (if (not Positive)
    (`/Game/Blueprints/Components/BasicCharacterComponent.OffsetAdrenaline` (`self.Basic Character Component`) 40)
    (`self.PlayCameraShake` "/Game/Misc/CShake_Damage.CShake_Damage_C" 1.0)
    (if (== HealthPercent 0.0)
      (`self.PlaySoundAtLocation` "/Game/SFX/SC_DEATH.SC_DEATH"
        (:`Out`
          (`self.DisableInput` (`GameplayStatics.GetPlayerController` 0))
          (`KismetSystemLibrary.Delay` 2.0)
          (`GameplayStatics.OpenLevel` "L_GameWorld")))
      (else
        (`self.PlaySoundAtLocation` "/Game/SFX/SC_PAIN.SC_PAIN")))))

(event `self.Basic Character Component.OnStaminaUpdate`
  (params (CurrentStamina :type Integer) (StaminaPercent :type "Float (double-precision)") (Positive :type Boolean))
  (`self.UpdateStaminaFeedback` StaminaPercent)
  (`self.SetPlayerSpeed`))

(event `self.Basic Character Component.OnFall`
  (params (Distance :type "Float (double-precision)"))
  (`self.PlaySoundAtLocation` "/Game/SFX/SC_FALL.SC_FALL"))

(event `Dodge`
  (if (and (> (`self.GetVelocityLength`) 0.0) (not (`NavMovementComponent.IsFalling` (`self.CharacterMovement`))) (`self.CanDodge`))
    (`|ExecutionSequence`
      (:`then_0`
        (`KismetSystemLibrary.MoveComponentTo` (`self.CapsuleComponent`) (`self.GetDodgeLocation`) (`self.K2_GetActorRotation`) true false 0.2 true))
      (:`then_1`
        (`/Game/Blueprints/Components/BasicCharacterComponent.OffsetStamina` (`self.Basic Character Component`) -15)
        (`self.StopStaminaRegen` 1.5)
        (`self.PlayCameraShake` "/Game/Misc/CShake_Dodge.CShake_Dodge_C" 1.0)
        (`self.PlaySoundAtLocation` "/Game/SFX/SC_DODGE.SC_DODGE"
          (:`Out`
            (set `self.CanDodge` false)
            (`KismetSystemLibrary.Delay` 1.0)
            (set `self.CanDodge` true)))))))

(event `InputAction|Dodge`
  (params (Key :type "Key Structure"))
  (:`Pressed`
    (`self.Dodge`)))

(event `InputAction|Inventory`
  (params (Key :type "Key Structure"))
  (:`Pressed`
    (`/Game/Blueprints/Components/InventoryComponent.OpenInventory` (`self.InventoryComponent`) "NewEnumerator0")))

(event `self.InventoryComponent.OnInventoryOpen`
  (bind _playercontroller (`self.PlayerController`))
  (`/Game/Blueprints/BP_PlayerController.SetHUDVisibility` _playercontroller "Collapsed")
  (`self.DisableInput` _playercontroller))

(event `self.InventoryComponent.OnInventoryClose`
  (bind _playercontroller (`self.PlayerController`))
  (`/Game/Blueprints/BP_PlayerController.SetHUDVisibility` _playercontroller "Visible")
  (`self.EnableInput` _playercontroller))

(event `self.Basic Character Component.OnAdrenalineUpdate`
  (params (Percentage :type "Float (double-precision)"))
  (bind _sc_heartbeat (`self.SC_HEARTBEAT`))
  (`AudioComponent.SetVolumeMultiplier` _sc_heartbeat Percentage)
  (`AudioComponent.SetPitchMultiplier` _sc_heartbeat (+ Percentage 0.9))
  (`self.SetPlayerSpeed`)
  (bind (_direction _alpha) (`Timeline|Timeline_FOV` :!via `PlayFromStart`)
    (:`Update`
      (`self.SetFOV` (`KismetMathLibrary.Lerp` 0.0 (`KismetMathLibrary.Conv_IntToDouble` (`KismetMathLibrary.FFloor` (* Percentage 5.0))) _alpha)))))

(event `StartAdrenalineTimer`
  (bind _returnvalue (`KismetSystemLibrary.K2_SetTimerDelegate` (delegate `DecreaseAdrenaline`) 0.35 true))
  (set `self.Timer_Adrenaline` _returnvalue))

(event `DecreaseAdrenaline`
  (`/Game/Blueprints/Components/BasicCharacterComponent.OffsetAdrenaline` (`self.Basic Character Component`) -1))

(fn `FindInteractionActor`
  (returns (Actor :type "Actor Object Reference"))
  (bind _returnvalue (`SceneComponent.K2_GetComponentLocation` (`self.PlayerCamera`)))
  (bind _outhit (`KismetSystemLibrary.LineTraceSingle` :`Start` _returnvalue :`End` (+ _returnvalue (* (`KismetMathLibrary.GetForwardVector` (`self.GetControlRotation`)) (`self.SearchRange`))) :`TraceChannel` "TraceTypeQuery1" :`DrawTime` 2.0))
  (return (`.HitActor` (`GameplayStatics.BreakHitResult` _outhit))))

(fn `GetDodgeLocation`
  (returns (ReturnValue :type "Vector Structure"))
  (bind _returnvalue (`self.K2_GetActorLocation`))
  (bind (_returnvalue_roll _returnvalue_pitch _returnvalue_yaw) (`KismetMathLibrary.BreakRotator` (`KismetMathLibrary.Conv_VectorToRotator` (`self.GetVelocity`))))
  (bind _returnvalue_2 (`KismetMathLibrary.GetForwardVector` (`KismetMathLibrary.MakeRotator` 0.0 0.0 _returnvalue_yaw)))
  (bind _returnvalue_3 (* (`.DodgeRange_2_682362704EA2494CC1A1CFAB46AF9BA1` (break `/Game/Data/STRUCT_PlayerStatus` (`self.PlayerStatus`))) (`self.GetFromPercentRange` (`/Game/Blueprints/Components/BasicCharacterComponent.GetStaminaPercent` (`self.Basic Character Component`)) 0.5 1.0)))
  (bind _outhit (`KismetSystemLibrary.LineTraceSingle` (- _returnvalue (0.0 0.0 80.0)) (+ _returnvalue (* _returnvalue_2 _returnvalue_3) (0.0 0.0 -80.0)) "TraceTypeQuery1"))
  (bind (_bblockinghit _binitialoverlap _time _distance _location _impactpoint _normal) (`GameplayStatics.BreakHitResult` _outhit))
  (return (+ (* _returnvalue_2 (`KismetMathLibrary.SelectFloat` _distance _returnvalue_3 _bblockinghit)) (`self.K2_GetActorLocation`) (`KismetMathLibrary.SelectVector` (* _normal (`KismetSystemLibrary.MakeLiteralDouble` (`CapsuleComponent.CapsuleRadius` (`self.CapsuleComponent`)))) (0.0 0.0 0.0) _bblockinghit))))

(fn `GetFOV`
  (returns (FOV :type "Float (double-precision)"))
  (return (`.FOV_15_9A758EB84916A9EFFD47BEA7298FCEC0` (break `/Game/Data/STRUCT_GameSettings` (`self.GameSettings`)))))

(fn `GetMaterialSound`
  (returns (Sound :type "SoundCue Object Reference"))
  (bind _returnvalue (`self.K2_GetActorLocation`))
  (bind _outhit (`KismetSystemLibrary.LineTraceSingle` :`Start` (+ _returnvalue (0.0 0.0 30.0)) :`End` (+ _returnvalue (0.0 0.0 -100.0)) :`TraceChannel` "TraceTypeQuery1" :`DrawTime` 1.0))
  (return (select `EPhysicalSurface` (`GameplayStatics.GetSurfaceType` _outhit) :`SurfaceType_Default` "/Game/SFX/SC_FS_CONCRETE.SC_FS_CONCRETE" :`SurfaceType1` "/Game/SFX/SC_FS_MUD.SC_FS_MUD" :`SurfaceType2` "/Game/SFX/SC_FS_CONCRETE.SC_FS_CONCRETE" :`SurfaceType3` "/Game/SFX/SC_FS_WATER.SC_FS_WATER" :!type "SoundCue Object Reference")))

(fn `GetMaxSpeed`
  (returns (MaxSpeed :type "Float (double-precision)"))
  (return (`.MaxSpeed_10_D632E689418488BBC2E5D897DDC19FB1` (break `/Game/Data/STRUCT_PlayerStatus` (`self.PlayerStatus`)))))

(fn `RetrieveSavedData`
  (params (Inventory :type "Array of /Game/Data/STRUCT_InventoryItem Structure"))
  (`/Game/Blueprints/Components/InventoryComponent.SetInventory` (`self.InventoryComponent`) Inventory))

(fn `SetFOV`
  (params (Offset :type "Float (double-precision)"))
  (`CameraComponent.SetFieldOfView` (`self.PlayerCamera`) (+ Offset (`self.GetFOV`))))

(fn `SetPlayerSpeed`
  (bind _basic_character_component (`self.Basic Character Component`))
  (set `CharacterMovementComponent.MaxWalkSpeed` (`KismetMathLibrary.FClamp` (+ (* (`/Game/Blueprints/Components/BasicCharacterComponent.GetStaminaPercent` _basic_character_component) 50.0) (* (`/Game/Blueprints/Components/BasicCharacterComponent.GetAdrenalinePercent` _basic_character_component) 100.0) (`self.GetBaseSpeed`)) 0.0 (`self.GetMaxSpeed`)) (`self.CharacterMovement`)))

(fn `UpdateHealthFeedback`
  (params (`Health Percent` :type "Float (double-precision)"))
  (bind _returnvalue (- 1.0 `Health Percent`))
  (bind _gamefeedbackpp (`self.GameFeedbackPP`))
  (bind (_x _y _z _w) (`KismetMathLibrary.BreakVector4` (`.ColorGamma` (break `PostProcessSettings` (`PostProcessComponent.Settings` _gamefeedbackpp)))))
  (set `PostProcessComponent.Settings` (make `PostProcessSettings` :`ColorGamma` (`KismetMathLibrary.MakeVector4` (+ _returnvalue 1.0) _y _z _w) :`SceneFringeIntensity` (* _returnvalue 5.0)) _gamefeedbackpp))

(fn `UpdateStaminaFeedback`
  (params (StaminaPercent :type "Float (double-precision)"))
  (bind _returnvalue (`self.GetFromPercentRange` StaminaPercent 0.25 1.0))
  (bind _gamefeedbackpp (`self.GameFeedbackPP`))
  (bind ((`ColorSaturation` _colorsaturation) (`ColorGamma` _colorgamma) (`SceneFringeIntensity` _scenefringeintensity)) (break `PostProcessSettings` (`PostProcessComponent.Settings` _gamefeedbackpp)))
  (bind (_x _y _z) (`KismetMathLibrary.BreakVector4` _colorsaturation))
  (bind (_x_2 _y_2 _z_2) (`KismetMathLibrary.BreakVector4` _colorgamma))
  (set `PostProcessComponent.Settings` (make `PostProcessSettings` :`ColorSaturation` (`KismetMathLibrary.MakeVector4` _x _y _z _returnvalue) :`ColorGamma` (`KismetMathLibrary.MakeVector4` _x_2 _y_2 _z_2 _returnvalue) :`SceneFringeIntensity` _scenefringeintensity) _gamefeedbackpp))

(fn `UserConstructionScript`)