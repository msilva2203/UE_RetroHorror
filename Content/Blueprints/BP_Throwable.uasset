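; Throwable physics prop that the player picks up through its InteractionComponent, holds at the ThrowableLocation, then throws or drops.
; Throw re-enables physics with a velocity-change impulse and flags it as thrown, so hits stun IF_Damage actors.
; Impact sounds are gated by a startup delay and distance from the last sounded hit.
; An overlap volume makes the mesh ignore the Pawn channel while the player overlaps it.
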(event `self.ReceiveBeginPlay`
  (`/Game/Blueprints/Components/InteractionComponent.Setup` (`self.InteractionComponent`) (`self.Name`) "NewEnumerator5")
  (`KismetSystemLibrary.Delay` 2.0)
  (set `self.CanHit` true))

(event `/Game/Blueprints/Interfaces/IF_Interaction.OpenInteraction`
  (`self.EnableInput` (`GameplayStatics.GetPlayerController` 0))
  (if (not (`KismetSystemLibrary.IsValid` (`self.PlayerCharacter`)))
    (set `self.PlayerCharacter` (cast `/Game/Blueprints/BP_PlayerCharacter` (`GameplayStatics.GetPlayerPawn` 0) :!pure true))))

(event `/Game/Blueprints/Interfaces/IF_Interaction.CloseInteraction`
  (`self.DisableInput` (`GameplayStatics.GetPlayerController` 0)))

(event `InputAction|Interaction`
  (params (Key :type "Key Structure"))
  (:`Pressed`
    (if (not (`self.bPickedUp`))
      (set `self.HasBeenThrown` false)
      (`PrimitiveComponent.SetSimulatePhysics` (`self.StaticMesh`) false)
      (`SceneComponent.K2_AttachToComponent` (`self.StaticMesh`) (`/Game/Blueprints/BP_PlayerCharacter.ThrowableLocation` (`self.PlayerCharacter`)) "None" "SnapToTarget" "SnapToTarget" "SnapToTarget" true)
      (`/Game/Blueprints/BP_PlayerCharacter.SetIsHoldingObject` (`self.PlayerCharacter`) true self)
      (`self.SetIsPickedUp` true))))

(event `/Game/Blueprints/Interfaces/IF_Damage.Impulse`
  (params (Direction :type "Vector Structure") (Force :type "Float (double-precision)"))
  (`PrimitiveComponent.AddImpulse` (`self.StaticMesh`) (* Direction Force) "None" true))

(event `self.StaticMesh.OnComponentHit`
  (params (HitComponent :type "PrimitiveComponent Object Reference") (OtherActor :type "Actor Object Reference") (OtherComp :type "PrimitiveComponent Object Reference") (NormalImpulse :type "Vector Structure") (Hit :type "HitResult Structure (by ref)"))
  (bind (_bblockinghit _binitialoverlap _time _distance _location _impactpoint _normal _impactnormal _physmat _hitactor) (`GameplayStatics.BreakHitResult` Hit))
  (`|ExecutionSequence`
    (:`then_0`
      (if (and (>= (`KismetMathLibrary.Vector_Distance` _location (`self.HitLocation`)) 100.0) (`self.CanHit`))
        (set `self.HitLocation` _location)
        (`GameplayStatics.PlaySoundAtLocation` (`self.SFX_Impact`) _impactpoint (struct) 1.0 1.0 0.0 null null null null)
        (`KismetSystemLibrary.PrintString` "Hit")))
    (:`then_1`
      (if (and (`KismetSystemLibrary.DoesImplementInterface` _hitactor "/Game/Blueprints/Interfaces/IF_Damage.IF_Damage_C") (`self.HasBeenThrown`))
        (message `/Game/Blueprints/Interfaces/IF_Damage.Stun` _hitactor (`self.Stun Time`))))))

(event `self.PlayerOverlapCollsiion.OnComponentBeginOverlap`
  (params (OverlappedComponent :type "PrimitiveComponent Object Reference") (OtherActor :type "Actor Object Reference") (OtherComp :type "PrimitiveComponent Object Reference") (OtherBodyIndex :type Integer) (bFromSweep :type Boolean) (SweepResult :type "HitResult Structure (by ref)"))
  (if (== OtherActor (`GameplayStatics.GetPlayerPawn` 0))
    (`PrimitiveComponent.SetCollisionResponseToChannel` (`self.StaticMesh`) "ECC_Pawn" "ECR_Ignore")))

(event `self.PlayerOverlapCollsiion.OnComponentEndOverlap`
  (params (OverlappedComponent :type "PrimitiveComponent Object Reference") (OtherActor :type "Actor Object Reference") (OtherComp :type "PrimitiveComponent Object Reference") (OtherBodyIndex :type Integer))
  (if (== OtherActor (`GameplayStatics.GetPlayerPawn` 0))
    (`PrimitiveComponent.SetCollisionResponseToChannel` (`self.StaticMesh`) "ECC_Pawn" "ECR_Block")))

(event `OnThrown`
  (set `self.HasBeenThrown` true)
  (`KismetSystemLibrary.Delay` 2.0)
  (set `self.HasBeenThrown` false))

(fn `Leave`
  (`self.K2_DetachFromActor` "KeepWorld" "KeepWorld" "KeepWorld")
  (`PrimitiveComponent.SetSimulatePhysics` (`self.StaticMesh`) true)
  (`self.SetIsPickedUp` false))

(fn `SetIsPickedUp`
  (params (bPickedUp :type Boolean))
  (bind _output_get (set `self.bPickedUp` bPickedUp))
  (`/Game/Blueprints/Components/InteractionComponent.SetIsActive` (`self.InteractionComponent`) (not _output_get)))

(fn `Throw`
  (params (Direction :type "Vector Structure") (Strength :type "Float (double-precision)"))
  (`PrimitiveComponent.SetSimulatePhysics` (`self.StaticMesh`) true)
  (`PrimitiveComponent.AddImpulse` (`self.StaticMesh`) (* Direction Strength) "None" true)
  (`self.SetIsPickedUp` false)
  (`PrimitiveComponent.SetCollisionResponseToChannel` (`self.StaticMesh`) "ECC_Pawn" "ECR_Block")
  (set `self.HasBeenThrown` true))

(fn `UserConstructionScript`)