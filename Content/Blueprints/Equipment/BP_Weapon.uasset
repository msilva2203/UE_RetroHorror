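; Equippable player hitscan weapon with semi or full-auto fire, recoil and ammo stored as the weapon item's quantity in the player's inventory.
; Shots trace from the camera with movement-based offset, sending damage and impulse through IF_Damage, or spawning decals and surface sounds on other hits.
; A release delay gates fire rate and chains automatic shots.
; Timed reloads repeatedly pull ammo items until full, interrupted by firing or unequipping.
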(event `self.ReceiveBeginPlay`
  (`parent.ReceiveBeginPlay`)
  (add `self.OnEquipped` (delegate `OnEquip`))
  (add `self.OnUnequipped` (delegate `OnUnequip`)))

(event `OnEquip`
  (bind _returnvalue (`self.GetPlayerInventory`))
  (bind _weaponitem (`self.WeaponItem`))
  (if (`/Game/Blueprints/Components/InventoryComponent.HasItem` _returnvalue _weaponitem)
    (bind _output_get (set `self.Ammo` (`.Quantity` (`/Game/Blueprints/Components/InventoryComponent.GetItemQuantity` _returnvalue _weaponitem))))
    (if (> _output_get (`self.MaxAmmo`))
      (`/Game/Blueprints/Components/InventoryComponent.AddToInventory` (`self.GetPlayerInventory`) (`self.AmmoItem`) (- (`self.Ammo`) (`self.MaxAmmo`)))
      (`self.SetAmmo` (`self.MaxAmmo`)))))

(event `OnUnequip`
  (bind _returnvalue (`self.GetPlayerInventory`))
  (if (`/Game/Blueprints/Components/InventoryComponent.HasItem` _returnvalue (`self.WeaponItem`))
    (`/Game/Blueprints/Components/InventoryComponent.SetItemQuantity` _returnvalue (`self.WeaponItem`) (`self.Ammo`))
    (`self.InterruptReload`)))

(event `self.ReceiveTick`
  (params (DeltaSeconds :type "Float (single-precision)"))
  (`parent.ReceiveTick` DeltaSeconds))

(event `InputAction|Attack`
  (params (Key :type "Key Structure"))
  (:`Pressed`
    (set `self.HoldingFire` true)
    (`self.InterruptReload`)
    (`self.Shoot`))
  (:`Released`
    (set `self.HoldingFire` false)))

(event `InputAction|Reload`
  (params (Key :type "Key Structure"))
  (:`Pressed`
    (`self.Reload`)))

(event `Shoot`
  (if (and (not (`self.Blocked`)) (not (`self.IsReloading`)))
    (if (> (`self.Ammo`) 0)
      (`self.ReleaseFire` true)
      (`GameplayStatics.SpawnSoundAttached` (`self.SFX_Shooting`) (`self.WeaponBarrelLocation`) "None" (0.0 0.0 0.0) (struct) "KeepRelativeOffset" false 1.0 1.0 0.0 null null)
      (`self.SetAmmo` (- (`self.Ammo`) 1))
      (`self.AddRecoil`)
      (bind (_hit _distance _location _normal _hitactor _physmat) (`self.GetWeaponShotResult`))
      (if _hit
        (bind _miss (`self.DealDamage` _hitactor))
        (if _miss
          (`self.ShotFeedback` _location _normal _physmat)
          (else
            (`KismetSystemLibrary.PrintString` "WEAPON: Shooting")
            (`KismetSystemLibrary.DrawDebugSphere` _location 5.0 12 (struct :`G` 1.0 :`A` 1.0) 5.0))))
      (else
        (`self.ReleaseFire` false)
        (`GameplayStatics.SpawnSoundAttached` (`self.SFX_Empty`) (`self.WeaponBarrelLocation`) "None" (0.0 0.0 0.0) (struct) "KeepRelativeOffset" false 1.0 1.0 0.0 null null)))))

(event `ReleaseFire`
  (params (Shot :type Boolean))
  (if (not (`self.Blocked`))
    (set `self.Blocked` true)
    (if Shot
      (`GameplayStatics.SpawnSoundAttached` (`self.SFX_Release`) (`self.WeaponBarrelLocation`) "None" (0.0 0.0 0.0) (struct) "KeepRelativeOffset" false 1.0 1.0 0.0 null null))
    (`KismetSystemLibrary.Delay` (`self.ReleaseTime`))
    (set `self.Blocked` false)
    (if (and (`self.HoldingFire`) (`self.FullAuto`))
      (`self.Shoot`))))

(event `Reload`
  (if (< (`self.Ammo`) (`self.MaxAmmo`))
    (bind (_hasitem _quantity) (`self.HasAmmo`))
    (if _hasitem
      (set `self.IsReloading` true)
      (bind _returnvalue (`GameplayStatics.SpawnSoundAttached` (`self.SFX_Reload`) (`self.WeaponBarrelLocation`) "None" (0.0 0.0 0.0) (struct) "KeepRelativeOffset" false 1.0 1.0 0.0 null null))
      (set `self.InstReloadSound` _returnvalue)
      (bind _returnvalue_2 (`KismetSystemLibrary.K2_SetTimerDelegate` (delegate `FinishReload`) (`self.ReloadTime`)))
      (set `self.Timer_Reload` _returnvalue_2)
      (else
        (`KismetSystemLibrary.PrintString` "Player doesn t have ammo item")))))

(event `FinishReload`
  (bind _ammo (`self.GetReloadedAmmo` (stale `Reload` _quantity)))
  (`self.RemoveAmmoFromPlayer` _ammo)
  (`self.SetAmmo` (`KismetMathLibrary.Clamp` (+ _ammo (`self.Ammo`)) 0 (`self.MaxAmmo`)))
  (set `self.IsReloading` false)
  (`self.Reload`)
  (`KismetSystemLibrary.PrintString` (`KismetStringLibrary.Concat_StrStr` "AMMO: " (`KismetStringLibrary.Conv_IntToString` (`self.Ammo`)))))

(event `InterruptReload`
  (`KismetSystemLibrary.K2_ClearAndInvalidateTimerHandle` (`self.Timer_Reload`))
  (set `self.IsReloading` false)
  (`self.SafeStopSound` (`self.InstReloadSound`)))

(fn `AddRecoil`
  (bind _returnvalue (`GameplayStatics.GetPlayerPawn` 0))
  (bind _recoil___yaw (`self.Recoil - Yaw`))
  (`Pawn.AddControllerPitchInput` _returnvalue (`self.Recoil - Pitch`))
  (`Pawn.AddControllerYawInput` _returnvalue (`KismetMathLibrary.RandomFloatInRange` (* _recoil___yaw -1.0) _recoil___yaw)))

(fn `DealDamage`
  (params (`Hit Actor` :type "Actor Object Reference"))
  (returns (Miss :type Boolean))
  (bind _hit_actor (`local.Hit Actor`))
  (`/Engine/EditorBlueprintResources/StandardMacros.IsValid` `Hit Actor`
    (:`Is Valid`
      (if (`KismetSystemLibrary.DoesImplementInterface` (`local.Hit Actor`) "/Game/Blueprints/Interfaces/IF_Damage.IF_Damage_C")
        (message `/Game/Blueprints/Interfaces/IF_Damage.Impulse` _hit_actor (`KismetMathLibrary.GetForwardVector` (`Pawn.GetControlRotation` (`GameplayStatics.GetPlayerPawn` 0))) (`self.Force`))
        (message `/Game/Blueprints/Interfaces/IF_Damage.Damage` _hit_actor (`self.GetWeaponDamage`))
        (return false)
        (else
          _)))
    (:`Is Not Valid`
      _))
  (return true))

(fn `GetBarrelLocation`
  (returns (ReturnValue :type "Vector Structure"))
  (return (`SceneComponent.K2_GetComponentLocation` (`self.WeaponBarrelLocation`))))

(fn `GetInaccuracy`
  (returns (`Inaccuracy Vector` :type "Vector Structure"))
  (bind _returnvalue (`GameplayStatics.GetPlayerPawn` 0))
  (bind _returnvalue_2 (`self.GetVelocity` _returnvalue))
  (bind _speed (message `/Game/Blueprints/Interfaces/IF_Actions.GetSpeed` _returnvalue))
  (bind _returnvalue_3 (* (/ (`KismetMathLibrary.Dot_VectorVector` _returnvalue_2 (`self.GetActorRightVector` _returnvalue)) _speed) 100.0))
  (`KismetSystemLibrary.PrintString` (`KismetStringLibrary.Conv_DoubleToString` _returnvalue_3))
  (return (`KismetMathLibrary.MakeVector` _returnvalue_3 _returnvalue_3 (* (/ (`KismetMathLibrary.Dot_VectorVector` _returnvalue_2 (`self.GetActorForwardVector` _returnvalue)) _speed) 100.0))))

(fn `GetPlayerInventory`
  (returns (ReturnValue :type "/Game/Blueprints/Components/InventoryComponent Object Reference"))
  (return (`self.GetComponentByClass` (`GameplayStatics.GetPlayerPawn` 0) "/Game/Blueprints/Components/InventoryComponent.InventoryComponent_C")))

(fn `GetReloadedAmmo`
  (params (`Total Quantity` :type Integer))
  (returns (Ammo :type Integer))
  (if (>= (- `Total Quantity` (`self.ReloadSize`)) 0)
    (return (`self.ReloadSize`))
    (else
      (return (`local.Total Quantity`)))))

(fn `GetSurfaceSound`
  (params (Surface :type "EPhysicalSurface Enum" :default "SurfaceType_Default"))
  (returns (Sound :type "SoundCue Object Reference"))
  (return (select `EPhysicalSurface` Surface :!type "SoundCue Object Reference")))

(fn `GetWeaponDamage`
  (returns (Damage :type Integer))
  (return (`self.Damage`)))

(fn `GetWeaponShotResult`
  (returns (Hit :type Boolean) (Distance :type "Float (single-precision)") (Location :type "Vector Structure") (Normal :type "Vector Structure") (HitActor :type "Actor Object Reference") (PhysMat :type "PhysicalMaterial Object Reference"))
  (bind _returnvalue (`PlayerCameraManager.GetCameraLocation` (`GameplayStatics.GetPlayerCameraManager` 0)))
  (bind (_outhit _returnvalue_2) (`KismetSystemLibrary.LineTraceSingle` _returnvalue (+ _returnvalue (* (`KismetMathLibrary.GetForwardVector` (`Controller.GetControlRotation` (`GameplayStatics.GetPlayerController` 0))) (`self.Range`)) (`self.GetInaccuracy`)) "TraceTypeQuery4" false (`|MakeArray` (`GameplayStatics.GetPlayerPawn` 0) :!type "Actor Object Reference") "ForDuration"))
  (bind (_bblockinghit _binitialoverlap _time _distance _location _impactpoint _normal _impactnormal _physmat _hitactor _hitcomponent) (`GameplayStatics.BreakHitResult` _outhit))
  (`KismetSystemLibrary.PrintString` (`KismetSystemLibrary.GetDisplayName` _hitcomponent))
  (return _returnvalue_2 _distance _location _normal _hitactor _physmat))

(fn `HasAmmo`
  (returns (HasItem :type Boolean) (Quantity :type Integer))
  (bind (_has_item _quantity) (`/Game/Blueprints/Components/InventoryComponent.GetItemQuantity` (`self.GetPlayerInventory`) (`self.AmmoItem`)))
  (return _has_item _quantity))

(fn `RemoveAmmoFromPlayer`
  (params (Ammo :type Integer))
  (`/Game/Blueprints/Components/InventoryComponent.RemoveFromInventory` (`self.GetComponentByClass` (`GameplayStatics.GetPlayerPawn` 0) "/Game/Blueprints/Components/InventoryComponent.InventoryComponent_C") (`self.AmmoItem`) Ammo))

(fn `SetAmmo`
  (params (Ammo :type Integer))
  (bind _output_get (set `self.Ammo` Ammo))
  (`/Game/Blueprints/Components/InventoryComponent.SetItemQuantity` (`self.GetPlayerInventory`) (`self.WeaponItem`) _output_get))

(fn `ShotFeedback`
  (params (Location :type "Vector Structure") (Normal :type "Vector Structure") (PhysMaterial :type "PhysicalMaterial Object Reference"))
  (`GameplayStatics.SpawnDecalAtLocation` "/Game/Assets/ColdharbourSeaside/ColdharbourSeaside/Decals/Materials/MI_BloodSmears.MI_BloodSmears" (10.0 10.0 10.0) Location (`KismetMathLibrary.RotatorFromAxisAndAngle` Normal) 5.0)
  (`GameplayStatics.PlaySoundAtLocation` (`self.GetSurfaceSound` (select `bool` (`KismetSystemLibrary.IsValid` PhysMaterial) :`false` "SurfaceType_Default" :`true` (`PhysicalMaterial.SurfaceType` PhysMaterial))) (`local.Location`) (struct) 1.0 1.0 0.0 null null null null))

(fn `UserConstructionScript`)