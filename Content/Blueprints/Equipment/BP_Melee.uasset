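; BP_Melee is a melee equipment Blueprint that puts its skeletal mesh on the player's weapon mesh at BeginPlay.
; Attack runs a Visibility line trace from the camera along the control rotation up to Range, with persistent debug drawing left on.
; Hit actors implementing IF_Damage receive Damage through a DamageMessage interface call.
; GetAnimation picks a combo animation by wrapping the count with MaxCombo and clamping it to the Animations array.
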(event `self.ReceiveBeginPlay`
  (`SkinnedMeshComponent.SetSkinnedAssetAndUpdate` (`/Game/Blueprints/BP_PlayerCharacter.WeaponMesh` (`self.PlayerCharacter`)) (`self.SkeletalMesh`) true)
  (`KismetSystemLibrary.PrintString` "Melee equipment equiped"))

(event `Attack`
  (bind _returnvalue (`PlayerCameraManager.GetCameraLocation` (`GameplayStatics.GetPlayerCameraManager` 0)))
  (bind _outhit (`KismetSystemLibrary.LineTraceSingle` :`Start` _returnvalue :`End` (+ _returnvalue (* (`KismetMathLibrary.GetForwardVector` (`Controller.GetControlRotation` (`GameplayStatics.GetPlayerController` 0))) (`self.Range`))) :`TraceChannel` "TraceTypeQuery1" :`DrawDebugType` "Persistent"))
  (bind (_bblockinghit _binitialoverlap _time _distance _location _impactpoint _normal _impactnormal _physmat _hitactor) (`GameplayStatics.BreakHitResult` _outhit))
  (if (`KismetSystemLibrary.DoesImplementInterface` _hitactor "/Game/Blueprints/Interfaces/IF_Damage.IF_Damage_C")
    (message `/Game/Blueprints/Interfaces/IF_Damage.Damage` _hitactor (`self.Damage`))))

(fn `GetAnimation`
  (params (Combo :type Integer))
  (returns (Animation :type "AnimMontage Object Reference"))
  (return (`|GetArrayItem` (`self.Animations`) (`KismetMathLibrary.Clamp` (mod Combo (`self.MaxCombo`)) 0 (- (`KismetArrayLibrary.Array_Length` (`self.Animations`)) 1)))))

(fn `UserConstructionScript`)